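; Bush is a scavengeable plant that gives the player a random forage item the first time they touch it.
; When a "Body"-tagged component of a ThirdPersonCharacter overlaps its static mesh, it picks mushroom, cicada or berry at random.
; It increments that character's matching count, prints the item name, and clears its Scavengable flag so it yields nothing further.
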(event OnComponentBeginOverlap(StaticMeshComponent)
  (params (OverlappedComponent :type Primitive%20Component%20Object%20Reference) (OtherActor :type Actor%20Object%20Reference) (OtherComp :type Primitive%20Component%20Object%20Reference) (OtherBodyIndex :type Integer) (bFromSweep :type Boolean) (SweepResult :type Hit%20Result%20Structure%20%28by%20ref%29))
  (if (and (Variables|Default|GetScavengable) (Components|ComponentHasTag OtherComp "Body"))
    (bind _asthird_person_character (Utilities|Casting|CastToThirdPersonCharacter OtherActor))
    (switch int (Math|Random|RandomIntegerinRange 0 2)
      (:0
        (Math|Integer|IncrementInt (Variables|/Game/ThirdPersonBP/Blueprints/ThirdPersonCharacter.ThirdPersonCharacter_C|GetMushroomCount _asthird_person_character)
          (:%20%20
            (Development|PrintString "Mushroom"))))
      (:1
        (Math|Integer|IncrementInt (Variables|/Game/ThirdPersonBP/Blueprints/ThirdPersonCharacter.ThirdPersonCharacter_C|GetCicadaCount _asthird_person_character)
          (:%20%20
            (Development|PrintString "Cicada"))))
      (:2
        (Math|Integer|IncrementInt (Variables|/Game/ThirdPersonBP/Blueprints/ThirdPersonCharacter.ThirdPersonCharacter_C|GetBerryCount _asthird_person_character)
          (:%20%20
            (Development|PrintString "Berry")))))
    (Variables|Default|SetScavengable false)))

(fn ConstructionScript)