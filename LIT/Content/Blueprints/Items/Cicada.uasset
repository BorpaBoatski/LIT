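; Cicada is a timed lure actor that draws goon enemies to itself.
; Enemy_Goon_Base actors overlapping its sphere are added to an array and never removed on leaving.
; While its lifetime counts down, Tick rewrites each stored enemy's blackboard with the cicada as target, its location and an attracted flag.
; On expiry it clears target object and flag, calling DestroyActor inside that loop, or directly if none are stored.
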(event OnComponentBeginOverlap(Sphere2)
  (params (OverlappedComponent :type Primitive%20Component%20Object%20Reference) (OtherActor :type Actor%20Object%20Reference) (OtherComp :type Primitive%20Component%20Object%20Reference) (OtherBodyIndex :type Integer) (bFromSweep :type Boolean) (SweepResult :type Hit%20Result%20Structure%20%28by%20ref%29))
  ;[1 1 1] Add enemy into array
  (bind _asenemy_goon_base (Utilities|Casting|CastToEnemy_Goon_Base OtherActor))
  (Utilities|Array|Add (Variables|Default|GetAffected) _asenemy_goon_base))

(event Custom|LoseLife
  (params (Delta%20Seconds :type Float%20%28single-precision%29))
  ;[1 1 1] Lose life over time
  (Variables|Default|SetLifetime (- (Variables|Default|GetLifetime) Delta%20Seconds)))

(event Custom|End
  (bind _affected (Variables|Default|GetAffected))
  ;[1 1 1] Stop attracting
  (if (> (Utilities|Array|Length _affected) 0)
    (for _array_element _affected
      (AI|Components|Blackboard|SetValueasObject (AI|GetBlackboard _array_element) (Variables|Default|GetTargetObject) 0)
      (AI|Components|Blackboard|SetValueasBool (AI|GetBlackboard _array_element) (Variables|Default|GetAttracted) false)
      (Actor|DestroyActor))
    (else
      (Actor|DestroyActor))))

(event Custom|Attract
  ;[1 1 1] Attracted enemies
  (for _array_element (Variables|Default|GetAffected)
    (AI|Components|Blackboard|SetValueasObject (AI|GetBlackboard _array_element) (Variables|Default|GetTargetObject) self)
    (AI|Components|Blackboard|SetValueasBool (AI|GetBlackboard _array_element) (Variables|Default|GetAttracted) true)
    (AI|Components|Blackboard|SetValueasVector (AI|GetBlackboard _array_element) (Variables|Default|GetTargetLocation) (Transformation|GetActorLocation))))

(event EventTick
  (params (DeltaSeconds :type Float%20%28single-precision%29))
  (CallFunction|LoseLife DeltaSeconds)
  (if (<= (Variables|Default|GetLifetime) 0.0)
    (CallFunction|End)
    (elif (> (Utilities|Array|Length (Variables|Default|GetAffected)) 0)
      (CallFunction|Attract))))

(fn ConstructionScript)