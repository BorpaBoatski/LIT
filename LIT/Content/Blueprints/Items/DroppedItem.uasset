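; Dropped item actor that gives one of five item types to the ThirdPersonCharacter on overlap, then destroys itself.
; Shortly after BeginPlay, a timer calls SwitchMesh to set the mesh matching Item and toggle its visibility, printing the type.
; CheckInventory checks the player's matching Has flag; if already held, PlayerIn makes Tick retry until the player can receive it or the overlap ends.
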(event OnComponentBeginOverlap(StaticMesh)
  (params (OverlappedComponent :type Primitive%20Component%20Object%20Reference) (OtherActor :type Actor%20Object%20Reference) (OtherComp :type Primitive%20Component%20Object%20Reference) (OtherBodyIndex :type Integer) (bFromSweep :type Boolean) (SweepResult :type Hit%20Result%20Structure%20%28by%20ref%29))
  ;[1 1 1] Collision
  (bind _asthird_person_character (Utilities|Casting|CastToThirdPersonCharacter OtherActor))
  (CallFunction|CheckInventory _asthird_person_character))

(event OnComponentEndOverlap(StaticMesh)
  (params (OverlappedComponent :type Primitive%20Component%20Object%20Reference) (OtherActor :type Actor%20Object%20Reference) (OtherComp :type Primitive%20Component%20Object%20Reference) (OtherBodyIndex :type Integer))
  ;[1 1 1] Collision
  (Utilities|Casting|CastToThirdPersonCharacter OtherActor)
  (Variables|Default|SetPlayerIn false))

(event EventBeginPlay
  ;[1 1 1] Change Item Mesh
  (Utilities|Time|SetTimerbyFunctionName 0 "SwitchMesh" 0.1))

(event EventTick
  (params (DeltaSeconds :type Float%20%28single-precision%29))
  (if (Variables|Default|GetPlayerIn)
    (bind _asthird_person_character (Utilities|Casting|CastToThirdPersonCharacter (Game|GetPlayerCharacter 0)))
    (CallFunction|CheckInventory _asthird_person_character)))

(fn ConstructionScript)

(fn SwitchMesh
  (bind _staticmesh (Variables|Default|GetStaticMesh))
  (bind _item (Variables|Default|GetItem))
  (Development|PrintString (Utilities|String|ToString(Integer) _item))
  (switch int _item
    (:Default
      (Components|StaticMesh|SetStaticMesh _staticmesh "/Game/Geometry/Items/Item_Berry.Item_Berry" :!label _label))
    (:0
      (goto _label))
    (:1
      (Components|StaticMesh|SetStaticMesh _staticmesh "/Game/Geometry/Items/Item_IronBody.Item_IronBody"))
    (:2
      (Components|StaticMesh|SetStaticMesh _staticmesh "/Game/Geometry/Items/Item_SleepPowder.Item_SleepPowder"))
    (:3
      (Components|StaticMesh|SetStaticMesh _staticmesh "/Game/Geometry/Items/Item_Cicada.Item_Cicada"))
    (:4
      (Components|StaticMesh|SetStaticMesh _staticmesh "/Game/Geometry/Items/Item_Shroom.Item_Shroom")))
  (Rendering|ToggleVisibility (Variables|Default|GetStaticMesh) false))

(fn CheckInventory
  (params (Player :type Third%20Person%20Character%20Object%20Reference))
  (switch int (Variables|Default|GetItem)
    (:Default
      (if (Variables|/Game/ThirdPersonBP/Blueprints/ThirdPersonCharacter.ThirdPersonCharacter_C|GethasBerry Player) :!label _label
        (Variables|Default|SetPlayerIn true :!label _label_2)
        (else
          (Default|ReceiveItem Player (Variables|Default|GetItem) :!label _label_3)
          (Actor|DestroyActor))))
    (:0
      (goto _label))
    (:1
      (if (Variables|/Game/ThirdPersonBP/Blueprints/ThirdPersonCharacter.ThirdPersonCharacter_C|GethasIronBody Player)
        (goto _label_2)
        (else
          (goto _label_3))))
    (:2
      (if (Variables|/Game/ThirdPersonBP/Blueprints/ThirdPersonCharacter.ThirdPersonCharacter_C|GethasPowder Player)
        (goto _label_2)
        (else
          (goto _label_3))))
    (:3
      (if (Variables|/Game/ThirdPersonBP/Blueprints/ThirdPersonCharacter.ThirdPersonCharacter_C|GethasCicada Player)
        (goto _label_2)
        (else
          (goto _label_3))))
    (:4
      (if (Variables|/Game/ThirdPersonBP/Blueprints/ThirdPersonCharacter.ThirdPersonCharacter_C|GethasMushroom Player)
        (goto _label_2)
        (else
          (goto _label_3))))))