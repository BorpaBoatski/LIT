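; Enemy01 is a simple enemy actor that chases the player pawn and destroys it on overlap.
; BeginPlay caches the first player's pawn, and each Tick turns the actor to face it, then steps along the forward vector by Speed.
; Movement sets location directly without sweep or delta-time scaling, so pace depends on frame rate.
; Destroying the player clears the cached reference.
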(event EventBeginPlay
  ;[1 1 1] GetPlayerActor
  (Variables|Default|SetPlayer (Game|Player|GetPlayerPawn 0)))

(event Collision|EventActorBeginOverlap
  (params (OtherActor :type Actor%20Object%20Reference))
  ;[1 1 1] Destroy Player on overlap
  (if (== OtherActor (Variables|Default|GetPlayer))
    (Actor|DestroyActor OtherActor)
    (Variables|Default|SetPlayer 0)))

(event EventTick
  (params (DeltaSeconds :type Float%20%28single-precision%29))
  (bind _returnvalue (Transformation|GetActorRotation))
  (bind _player (Variables|Default|GetPlayer))
  (bind (_roll _pitch _yaw) (Math|Rotator|BreakRotator _returnvalue))
  (if (!= _player 0)
    ;[1 1 1] Actor look at Player
    (Transformation|SetActorRotation (Math|Rotator|FindLookatRotation (Transformation|GetActorLocation) (Transformation|GetActorLocation _player)))
    ;[1 1 1] Actor move to Player
    (Transformation|SetActorLocation (+ (Transformation|GetActorLocation) (* (Math|Vector|GetForwardVector (Math|Rotator|MakeRotator 0.0 _pitch _yaw)) (Variables|Default|GetSpeed))) false false)))

(fn ConstructionScript)