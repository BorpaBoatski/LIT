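; Placeholder tutorial actor that shows world-space text for the Sifu, totem and purple flower interactions.
; On BeginPlay it caches the player character, then every Tick rotates each remaining text component to face that player.
; A shared cleanup branch polls per-item interaction flags and destroys the matching text once its flag is true.
; The graph only reads these flags and never sets them.
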(event EventTick
  (params (DeltaSeconds :type Float%20%28single-precision%29))
  (bind _purple_flower_text_render (Variables|Default|GetPurple%20Flower%20Text%20Render))
  (bind _player (Variables|Default|GetPlayer))
  (bind _sifu_text_render (Variables|Default|GetSifu%20Text%20Render))
  (bind _totem_text_render (Variables|Default|GetTotem%20Text%20Render))
  (bind _purple_flower_text_render_2 (Variables|Default|GetPurple%20Flower%20Text%20Render))
  (bind _totem_text_render_2 (Variables|Default|GetTotem%20Text%20Render))
  (bind _sifu_text_render_2 (Variables|Default|GetSifu%20Text%20Render))
  (bind _returnvalue (Transformation|GetActorLocation _player))
  (Utilities|FlowControl|Sequence
    (:then_0
      (Utilities|IsValid _totem_text_render_2
        (:Is%20Valid
          (Transformation|SetWorldRotation _totem_text_render_2 (Math|Rotator|FindLookatRotation (Transformation|GetWorldLocation _totem_text_render_2) _returnvalue) false false))))
    (:then_1
      (Utilities|IsValid _sifu_text_render_2
        (:Is%20Valid
          (Transformation|SetWorldRotation _sifu_text_render_2 (Math|Rotator|FindLookatRotation (Transformation|GetWorldLocation _sifu_text_render_2) _returnvalue) false false))))
    (:then_2
      (Utilities|IsValid _purple_flower_text_render
        (:Is%20Valid
          (Transformation|SetWorldRotation _purple_flower_text_render (Math|Rotator|FindLookatRotation (Transformation|GetWorldLocation _purple_flower_text_render) _returnvalue) false false)))))
  (Utilities|FlowControl|Sequence
    (:then_0
      (if (Variables|Default|GetHasSifuInteracted)
        (Utilities|IsValid _sifu_text_render
          (:Is%20Valid
            (Components|DestroyComponent _sifu_text_render)))))
    (:then_1
      (if (Variables|Default|GetHasTotemInteracted)
        (Utilities|IsValid _totem_text_render
          (:Is%20Valid
            (Components|DestroyComponent _totem_text_render)))))
    (:then_2
      (if (Variables|Default|GetHasPurpFlowerInteracted)
        (Utilities|IsValid _purple_flower_text_render_2
          (:Is%20Valid
            (Components|DestroyComponent _purple_flower_text_render_2)))))))

(event EventBeginPlay
  (Variables|Default|SetPlayer (Game|GetPlayerCharacter 0)))

(fn ConstructionScript)