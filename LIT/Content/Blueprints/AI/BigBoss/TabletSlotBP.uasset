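; Tablet slot actor in the BigBoss folder that displays a tablet when one is slotted.
; SlotTablet clears CanBeSlotted, increments the shared tablet count on SKFB, then reveals the Tablet mesh with the material matching counts one to four.
; Box begin and end overlaps with ThirdPersonCharacter both enable input on the slot.
; The event graph's guarded call to SlotTablet is unconnected, so nothing here triggers slotting.
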(event OnComponentBeginOverlap(Box)
  (params (OverlappedComponent :type Primitive%20Component%20Object%20Reference) (OtherActor :type Actor%20Object%20Reference) (OtherComp :type Primitive%20Component%20Object%20Reference) (OtherBodyIndex :type Integer) (bFromSweep :type Boolean) (SweepResult :type Hit%20Result%20Structure%20%28by%20ref%29))
  (Utilities|Casting|CastToThirdPersonCharacter OtherActor)
  (Input|EnableInput (Game|GetPlayerController 0)))

(event OnComponentEndOverlap(Box)
  (params (OverlappedComponent :type Primitive%20Component%20Object%20Reference) (OtherActor :type Actor%20Object%20Reference) (OtherComp :type Primitive%20Component%20Object%20Reference) (OtherBodyIndex :type Integer))
  (Utilities|Casting|CastToThirdPersonCharacter OtherActor)
  (Input|EnableInput (Game|GetPlayerController 0)))

(event Input|KeyboardEvents|E
  (params (Key :type Key%20Structure)))

(fn ConstructionScript)

(fn SlotTablet
  (bind _tablet (Variables|Default|GetTablet))
  (bind _sk_fb (Variables|Default|GetSK_FB))
  (Variables|Default|SetCanBeSlotted false)
  (bind _output_get (Variables|/Game/Blueprints/AI/BigBoss/SK_FB.SK_FB_C|SetINT_TabletCount _sk_fb (+ (Variables|/Game/Blueprints/AI/BigBoss/SK_FB.SK_FB_C|GetINT_TabletCount _sk_fb) 1)))
  (if (== _output_get 1)
    (Rendering|Material|SetMaterial _tablet 0 "/Game/Materials/Tablet_1.Tablet_1")
    (Rendering|SetVisibility (Variables|Default|GetTablet) true false :!label _label)
    (elif (== _output_get 2)
      (Rendering|Material|SetMaterial _tablet 0 "/Game/Materials/Tablet_2.Tablet_2")
      (goto _label)
      (elif (== _output_get 3)
        (Rendering|Material|SetMaterial _tablet 0 "/Game/Materials/Tablet_3.Tablet_3")
        (goto _label)
        (elif (== _output_get 4)
          (Rendering|Material|SetMaterial _tablet 0 "/Game/Materials/Tablet_4.Tablet_4")
          (goto _label)
          (else
            _)))))
  (return))