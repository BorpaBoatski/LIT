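; Sunflower interactible that, when lit by a light projectile, clears vines and activates a portal to the next level.
; A LightProjectile with SunflowerPower is consumed, animates the flower, turns it emissive, destroys the vine wall, opens the vine gate and enables the portal.
; BeginPlay async-loads the next level asset.
; The player's Body overlapping the portal box updates the CharacterData save object and opens that level by name.
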(event OnComponentBeginOverlap(Sunflower)
  (params (OverlappedComponent :type Primitive%20Component%20Object%20Reference) (OtherActor :type Actor%20Object%20Reference) (OtherComp :type Primitive%20Component%20Object%20Reference) (OtherBodyIndex :type Integer) (bFromSweep :type Boolean) (SweepResult :type Hit%20Result%20Structure%20%28by%20ref%29))
  ;[1 1 1] Sunflower Interact
  (if (not (Variables|Default|GetCanUsePortal))
    (bind _aslight_projectile (Utilities|Casting|CastToLightProjectile OtherActor))
    (if (Variables|/Game/ThirdPersonBP/Blueprints/LightProjectile.LightProjectile_C|GetSunflowerPower _aslight_projectile)
      (Components|Animation|PlayAnimation (Variables|Default|GetSunflower) "/Game/Models_Animations/Sunflower/sunflower_Animation_Anim.sunflower_Animation_Anim" false)
      (CallFunction|LightInteractReceive _aslight_projectile))))

(event OnComponentBeginOverlap(Box)
  (params (OverlappedComponent :type Primitive%20Component%20Object%20Reference) (OtherActor :type Actor%20Object%20Reference) (OtherComp :type Primitive%20Component%20Object%20Reference) (OtherBodyIndex :type Integer) (bFromSweep :type Boolean) (SweepResult :type Hit%20Result%20Structure%20%28by%20ref%29))
  ;[1 1 1] Check if player has come into contact with portal, if so teleports player to next level
  (if (Components|ComponentHasTag OtherComp "Body")
    (Utilities|Casting|CastToThirdPersonCharacter OtherActor)
    (if (Variables|Default|GetCanUsePortal)
      (CallFunction|UpdateCharacterData)
      (Game|OpenLevel(byName) (Utilities|String|StringToName (Utilities|GetDisplayName (Variables|Default|GetNextLevel)))))))

(event EventLightInteractReceive
  (params (LightProjectile :type Light%20Projectile%20Object%20Reference))
  ;[1 1 1] Changes Material of Sunflower to something more Emissive
  (Actor|DestroyActor LightProjectile)
  (Rendering|Material|SetMaterial (Variables|Default|GetSunflower) 0 "/Game/Materials/Sunflower/fpi_sunflower_inst_Emissive.fpi_sunflower_inst_Emissive")
  (Variables|Default|SetCanUsePortal true)
  ;[1 1 1] Destroys Vinewalls
  (Components|DestroyComponent (Variables|Default|GetVineWall))
  (Components|Animation|PlayAnimation (Variables|Default|GetVineGate) "/Game/Geometry/FPI_Vinegate_Shortcut_Anim_Activated_Anim.FPI_Vinegate_Shortcut_Anim_Activated_Anim" false) ; Open Vinegate
  ;[1 1 1] Plays sound upon lighting up Sunflower
  (Audio|PlaySound2D "/Game/Audio/NewSounds/SFX/Audio_Sunflower_Cue.Audio_Sunflower_Cue"))

(event Collision|EventActorBeginOverlap
  (params (OtherActor :type Actor%20Object%20Reference))
  ;[1 1 1] Override parent collision
)

(event EventBeginPlay
  ;[1 1 1] Prepare next level
  (bind _levelstream (Variables|Default|GetLevelStream)
    (:then
      (bind _object (Utilities|AsyncLoadAsset _levelstream)
        (:Completed
          (Variables|Default|SetNextLevel _object)
          (Development|PrintString "Next level ready"))))
    (:else
      (Development|PrintString "Sunflower: WARNING!! No level to stream"))))

(fn ConstructionScript)

(fn UpdateCharacterData
  (bind _asgame_instance_bp (Utilities|Casting|CastToGameInstance_BP (Game|GetGameInstance)))
  (bind _returnvalue (SaveGame|LoadGamefromSlot (Variables|/Game/Blueprints/SaveGames/GameInstance_BP.GameInstance_BP_C|GetCharacterDataName _asgame_instance_bp)))
  (bind _ascharacter_data_bp (Utilities|Casting|CastToCharacterData_BP _returnvalue))
  (bind _asthird_person_character (Utilities|Casting|CastToThirdPersonCharacter (Game|GetPlayerCharacter 0)))
  (Default|SetData _ascharacter_data_bp (Utilities|Struct|MakeS_MainCharacter (Variables|/Game/ThirdPersonBP/Blueprints/ThirdPersonCharacter.ThirdPersonCharacter_C|GetHealth _asthird_person_character) (Variables|/Game/ThirdPersonBP/Blueprints/ThirdPersonCharacter.ThirdPersonCharacter_C|GethasBerry _asthird_person_character) (Variables|/Game/ThirdPersonBP/Blueprints/ThirdPersonCharacter.ThirdPersonCharacter_C|GethasMushroom _asthird_person_character) (Variables|/Game/ThirdPersonBP/Blueprints/ThirdPersonCharacter.ThirdPersonCharacter_C|GethasCicada _asthird_person_character) (Variables|/Game/ThirdPersonBP/Blueprints/ThirdPersonCharacter.ThirdPersonCharacter_C|GethasIronBody _asthird_person_character) (Variables|/Game/ThirdPersonBP/Blueprints/ThirdPersonCharacter.ThirdPersonCharacter_C|GethasPowder _asthird_person_character) (Variables|Default|GetNextLevel)))
  (return false))