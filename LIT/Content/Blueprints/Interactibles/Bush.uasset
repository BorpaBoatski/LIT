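; Interactible bush that plays a rustle sound when overlapped and gives the player a one-time random scavenged item.
; On mesh overlap, if still scavengable and the overlapping component is tagged "Body", it casts the actor to ThirdPersonCharacter.
; A random pick increments that character's mushroom, cicada or berry count, prints it for debugging, then clears the Scavengable flag.
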(event OnComponentBeginOverlap(StaticMeshComponent)
  (params (OverlappedComponent :type Primitive%20Component%20Object%20Reference) (OtherActor :type Actor%20Object%20Reference) (OtherComp :type Primitive%20Component%20Object%20Reference) (OtherBodyIndex :type Integer) (bFromSweep :type Boolean) (SweepResult :type Hit%20Result%20Structure%20%28by%20ref%29))
  (Audio|PlaySoundatLocation "/Game/Audio/Interactibles/Audio_Bush_Cue.Audio_Bush_Cue" (Transformation|GetActorLocation self))
  (if (and (Variables|Default|GetScavengable) (Components|ComponentHasTag OtherComp "Body"))
    (bind _asthird_person_character (Utilities|Casting|CastToThirdPersonCharacter OtherActor))
    (switch int (Math|Random|RandomIntegerinRange 0 2)
      (:Default
        (bind _result (Math|Integer|IncrementInt (Variables|/Game/ThirdPersonBP/Blueprints/ThirdPersonCharacter.ThirdPersonCharacter_C|GetBerryCount _asthird_person_character) :!label _label)
          (:%20%20
            (Development|PrintString (Utilities|String|ToString(Integer) _result)))))
      (:0
        (bind _result_2 (Math|Integer|IncrementInt (Variables|/Game/ThirdPersonBP/Blueprints/ThirdPersonCharacter.ThirdPersonCharacter_C|GetMushroomCount _asthird_person_character))
          (:%20%20
            (Development|PrintString (Utilities|String|ToString(Integer) _result_2)))))
      (:1
        (bind _result_3 (Math|Integer|IncrementInt (Variables|/Game/ThirdPersonBP/Blueprints/ThirdPersonCharacter.ThirdPersonCharacter_C|GetCicadaCount _asthird_person_character))
          (:%20%20
            (Development|PrintString (Utilities|String|ToString(Integer) _result_3)))))
      (:2
        (goto _label)))
    (Variables|Default|SetScavengable false)))

(fn ConstructionScript)