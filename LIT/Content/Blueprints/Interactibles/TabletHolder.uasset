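; Interactible tablet holder that, once activated, rises with a sound and presents a bobbing tablet that opens an exit door.
; A looping timer drives TabletBobbing, which offsets the tablet vertically along a sine wave.
; The first ThirdPersonCharacter to overlap the capsule destroys the tablet, resets the bobbing timer, then slides ExitDoor by DoorMovement with a sound and destroys it.
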(event OnComponentBeginOverlap(Capsule)
  (params (OverlappedComponent :type Primitive%20Component%20Object%20Reference) (OtherActor :type Actor%20Object%20Reference) (OtherComp :type Primitive%20Component%20Object%20Reference) (OtherBodyIndex :type Integer) (bFromSweep :type Boolean) (SweepResult :type Hit%20Result%20Structure%20%28by%20ref%29))
  (bind _exitdoor (Variables|Default|GetExitDoor))
  (bind _rootcomponent (Variables|/Script/Engine.Actor|GetRootComponent _exitdoor))
  (bind _returnvalue (Transformation|GetWorldLocation _rootcomponent))
  ;[1 1 1] Open Door
  (Utilities|Casting|CastToThirdPersonCharacter OtherActor)
  (Utilities|FlowControl|DoOnce false
    (:Completed
      (Components|DestroyComponent (Variables|Default|GetTablet))
      (Utilities|Time|SetTimerbyFunctionName 0 "TabletBobbing" 0.0)
      (Audio|PlaySoundatLocation (Variables|Default|GetDoorSound) _returnvalue)
      (Components|MoveComponentTo _rootcomponent (+ _returnvalue (Variables|Default|GetDoorMovement)) (Transformation|GetWorldRotation _rootcomponent) false false 2.0 false)
      (Actor|DestroyActor (Variables|Default|GetExitDoor)))))

(event Custom|Activate
  (bind _returnvalue (Transformation|GetActorLocation))
  ;[1 1 1] Raise TabletHolder
  (Variables|Default|SetActivated true)
  (Audio|PlaySoundatLocation "/Game/Audio/NewSounds/SFX/Audio_complete_shrine_effect_Cue.Audio_complete_shrine_effect_Cue" _returnvalue)
  (Components|MoveComponentTo (Variables|Default|GetDefaultSceneRoot1) (+ _returnvalue "0, 0,280.000000") (Transformation|GetActorRotation) false false 2.0 false)
  (Utilities|Time|SetTimerbyFunctionName 0 "TabletBobbing" 0.1 true))

(fn ConstructionScript)

(fn TabletBobbing
  (Variables|Default|SetTimer (+ 1.0 (Variables|Default|GetTimer)))
  (Transformation|SetRelativeLocation (Variables|Default|GetTablet) (+ "0, 0,225.000000" (Math|Vector|MakeVector 0.0 0.0 (* (Math|Trig|Sin(Degrees) (Variables|Default|GetTimer)) 2e+01))) false false))