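; Trapdoor spider hazard that devours players or enemies that stay inside its detection box.
; An overlap while ready waits a short delay, then Devour teleports a still-present player to DeathZone and damages them, or destroys an Enemy-tagged actor.
; Each kill or player hit starts a cooldown that Tick counts down only while the zone is occupied.
; Re-arming does not recheck occupants, so only a new overlap triggers an attack.
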(event OnComponentBeginOverlap(DetectionBox)
  (params (OverlappedComponent :type Primitive%20Component%20Object%20Reference) (OtherActor :type Actor%20Object%20Reference) (OtherComp :type Primitive%20Component%20Object%20Reference) (OtherBodyIndex :type Integer) (bFromSweep :type Boolean) (SweepResult :type Hit%20Result%20Structure%20%28by%20ref%29))
  (Utilities|Array|Add (Variables|Default|GetInZone) OtherActor)
  (if (and (<= (Variables|Default|GetCanDevourTimer) 0.0) (Variables|Default|GetCanDevour))
    (Development|PrintString (Utilities|GetDisplayName OtherActor))
    (Utilities|FlowControl|Delay 2.0)
    (CallFunction|Devour OtherActor)))

(event OnComponentEndOverlap(DetectionBox)
  (params (OverlappedComponent :type Primitive%20Component%20Object%20Reference) (OtherActor :type Actor%20Object%20Reference) (OtherComp :type Primitive%20Component%20Object%20Reference) (OtherBodyIndex :type Integer))
  (Utilities|Array|RemoveItem (Variables|Default|GetInZone) OtherActor))

(event EventBeginPlay
  (Variables|Default|SetCanDevourTimer 0.0))

(event EventTick
  (params (DeltaSeconds :type Float%20%28single-precision%29))
  (if (> (Utilities|Array|Length (Variables|Default|GetInZone)) 0)
    (bind _output_get (Variables|Default|SetCanDevourTimer (- (Variables|Default|GetCanDevourTimer) DeltaSeconds)))
    (if (<= _output_get 0.0)
      (Variables|Default|SetCanDevourTimer 0.0)
      (Variables|Default|SetCanDevour true))))

(fn ConstructionScript)

(fn PlayerStrobe
  (Utilities|FlowControl|ForLoopwithBreak 0 0))

(fn Devour
  (params (OtherActor :type Actor%20Object%20Reference))
  (if (Utilities|Array|ContainsItem (Variables|Default|GetInZone) OtherActor)
    (if (Actor|ActorHasTag OtherActor "Player")
      (bind _asthird_person_character (Utilities|Casting|CastToThirdPersonCharacter OtherActor))
      (Transformation|SetActorLocation _asthird_person_character (+ (Transformation|GetWorldLocation (Variables|Default|GetDeathZone)) "0, 0, 0") false false)
      (Default|NewPlayerHealthManager _asthird_person_character -3.0)
      (Variables|Default|SetCanDevourTimer (Variables|Default|GetDevourCooldown) :!label _label)
      (Variables|Default|SetCanDevour false)
      (elif (Actor|ActorHasTag OtherActor "Enemy")
        (Actor|DestroyActor OtherActor)
        (goto _label)))
    (else
      (return))))