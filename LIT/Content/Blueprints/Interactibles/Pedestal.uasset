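; Interactive puzzle pedestal that the player rotates with E, tracking whether it sits at its correct position.
; Overlapping Box1 as the ThirdPersonCharacter enables input, and leaving disables it.
; Each press, when unlocked and not spinning, cycles Code through four states while the Spin timeline yaws the mesh, then plays a sound.
; Tick continuously sets Solved by comparing Code to RightCode.
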(event OnComponentBeginOverlap(Box1)
  (params (OverlappedComponent :type Primitive%20Component%20Object%20Reference) (OtherActor :type Actor%20Object%20Reference) (OtherComp :type Primitive%20Component%20Object%20Reference) (OtherBodyIndex :type Integer) (bFromSweep :type Boolean) (SweepResult :type Hit%20Result%20Structure%20%28by%20ref%29))
  (Utilities|Casting|CastToThirdPersonCharacter OtherActor)
  (Input|EnableInput (Game|GetPlayerController 0)))

(event OnComponentEndOverlap(Box1)
  (params (OverlappedComponent :type Primitive%20Component%20Object%20Reference) (OtherActor :type Actor%20Object%20Reference) (OtherComp :type Primitive%20Component%20Object%20Reference) (OtherBodyIndex :type Integer))
  (Utilities|Casting|CastToThirdPersonCharacter OtherActor)
  (Input|DisableInput (Game|GetPlayerController 0)))

(event EventTick
  (params (DeltaSeconds :type Float%20%28single-precision%29))
  (if (== (Variables|Default|GetCode) (Variables|Default|GetRightCode))
    (Variables|Default|SetSolved true)
    (else
      (Variables|Default|SetSolved false))))

(event Input|KeyboardEvents|E
  (params (Key :type Key%20Structure))
  (bind _staticmesh1 (Variables|Default|GetStaticMesh1))
  (bind _returnvalue (Transformation|GetWorldRotation _staticmesh1))
  (bind (_roll _pitch _yaw) (Math|Rotator|BreakRotator _returnvalue))
  (:Pressed
    (if (and (Math|Boolean|Equal(Boolean) (Variables|Default|GetLock) false) (Math|Boolean|Equal(Boolean) (Variables|Default|GetFinishSpin) true))
      (bind _result (Math|Integer|IncrementInt (Variables|Default|GetCode))
        (:%20%20
          (Variables|Default|SetCode (Math|Integer|%(Integer) _result 4))
          (Variables|Default|SetoldZ _yaw)
          (bind _rotation (Timeline|Spin PlayFromStart)
            (:Update
              (Variables|Default|SetFinishSpin false)
              (Transformation|SetWorldRotation (Variables|Default|GetStaticMesh1) (Math|Rotator|MakeRotator _roll _pitch (+ (Variables|Default|GetoldZ) _rotation)) false false))
            (:Finished
              (Variables|Default|SetFinishSpin true)
              ;[1 1 1] Rotate Sound being played
              (Audio|PlaySound2D "/Game/Audio/SFX/Interactibles/Audio_PuzzleRotate_Cue.Audio_PuzzleRotate_Cue"))))))))

(fn ConstructionScript)