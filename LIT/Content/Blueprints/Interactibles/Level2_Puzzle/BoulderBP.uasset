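; BoulderBP is the boulder in the Level 2 puzzle that moves across a grid of linked tiles.
; On BeginPlay it registers itself with every pressure plate and the player character.
; Directional move events look up the current tile's neighbour, then timelines lerp position and rotation, provided the tile allows entry.
; On arrival, the tile's GetNextTile can chain further moves, and OnEntered notifies the tile reached.
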(event Custom|MoveUp
  (bind _currenttile (Variables|Default|GetCurrentTile))
  (bind _neighbours (Variables|/Game/Blueprints/Interactibles/Level2_Puzzle/Tiles/Tile.Tile_C|GetNeighbours _currenttile))
  (bind _value (Utilities|Map|Find _neighbours "/Game/Blueprints/Interactibles/Level2_Puzzle/Base/Up.Up"))
  (if (Variables|Default|GetCanMoveOverride)
    (Utilities|IsValid (Variables|Default|GetTargetTile)
      (:Is%20Not%20Valid
        (Utilities|IsValid _value
          (:Is%20Valid
            (CallFunction|MovetoTile _value)
            (CallFunction|RotatetoDirection "/Game/Blueprints/Interactibles/Level2_Puzzle/Base/Up.Up")))))))

(event Custom|RotateToDirection
  (params (TargetDirection :type Direction%20Object%20Reference))
  (Utilities|IsValid TargetDirection
    (:Is%20Valid
      (Variables|Default|SetTargetDirection TargetDirection)
      (bind _rotatetrack (Timeline|RotateTimeline PlayFromStart)
        (:Update
          (Transformation|SetActorRotation (Math|Rotator|Lerp(Rotator) (Variables|/Game/Blueprints/Interactibles/Level2_Puzzle/Base/Direction.Direction_C|GetRotation (Variables|Default|GetCurrentDirection)) (Variables|/Game/Blueprints/Interactibles/Level2_Puzzle/Base/Direction.Direction_C|GetRotation (Variables|Default|GetTargetDirection)) _rotatetrack true)))
        (:Finished
          (Variables|Default|SetCurrentDirection (Variables|Default|GetTargetDirection))
          (Variables|Default|SetTargetDirection 0))))))

(event Custom|MoveRight
  (bind _currenttile (Variables|Default|GetCurrentTile))
  (bind _neighbours (Variables|/Game/Blueprints/Interactibles/Level2_Puzzle/Tiles/Tile.Tile_C|GetNeighbours _currenttile))
  (bind _value (Utilities|Map|Find _neighbours "/Game/Blueprints/Interactibles/Level2_Puzzle/Base/Right.Right"))
  (if (Variables|Default|GetCanMoveOverride)
    (Utilities|IsValid (Variables|Default|GetTargetTile)
      (:Is%20Not%20Valid
        (Utilities|IsValid _value
          (:Is%20Valid
            (CallFunction|MovetoTile _value)
            (CallFunction|RotatetoDirection "/Game/Blueprints/Interactibles/Level2_Puzzle/Base/Right.Right")))))))

(event Custom|MoveToTile
  (params (TargetTile :type Tile%20Object%20Reference))
  (Utilities|IsValid TargetTile
    (:Is%20Valid
      (if (Default|CanPlayerEnter TargetTile self (Variables|Default|GetCurrentTile))
        (Development|PrintString "Is Valid")
        (Variables|Default|SetTargetTile TargetTile)
        (bind _movetrack (Timeline|MoveTimeline PlayFromStart)
          (:Update
            (Transformation|SetActorLocation (Math|Vector|Lerp(Vector) (Transformation|GetActorLocation (Variables|Default|GetCurrentTile)) (Transformation|GetActorLocation (Variables|Default|GetTargetTile)) _movetrack) false false)
            (Development|PrintString (Utilities|GetDisplayName (Variables|Default|GetTargetTile))))
          (:Finished
            (Variables|Default|SetTemp (Variables|Default|GetCurrentTile))
            (Variables|Default|SetCurrentTile (Variables|Default|GetTargetTile))
            (bind _output_get (Variables|Default|SetTargetTile (Default|GetNextTile (Variables|Default|GetCurrentTile) self (Variables|Default|GetTemp))))
            (Utilities|IsValid _output_get
              (:Is%20Valid
                (if (Default|CanPlayerEnter _output_get self (Variables|Default|GetCurrentTile))
                  (CallFunction|MovetoTile _output_get)
                  (else
                    (Variables|Default|SetTargetTile 0))))
              (:Is%20Not%20Valid
                _))
            (Default|OnEntered (Variables|Default|GetCurrentTile) self (Variables|Default|GetTemp))))
        (else
          (Development|PrintString "Is Not Valid"))))
    (:Is%20Not%20Valid
      (Development|PrintString "Tile Not Valid"))))

(event Custom|MoveDown
  (bind _currenttile (Variables|Default|GetCurrentTile))
  (bind _neighbours (Variables|/Game/Blueprints/Interactibles/Level2_Puzzle/Tiles/Tile.Tile_C|GetNeighbours _currenttile))
  (bind _value (Utilities|Map|Find _neighbours "/Game/Blueprints/Interactibles/Level2_Puzzle/Base/Down.Down"))
  (if (Variables|Default|GetCanMoveOverride)
    (Utilities|IsValid (Variables|Default|GetTargetTile)
      (:Is%20Not%20Valid
        (Utilities|IsValid _value
          (:Is%20Valid
            (CallFunction|MovetoTile _value)
            (CallFunction|RotatetoDirection "/Game/Blueprints/Interactibles/Level2_Puzzle/Base/Down.Down")))))))

(event Custom|MoveLeft
  (bind _currenttile (Variables|Default|GetCurrentTile))
  (bind _neighbours (Variables|/Game/Blueprints/Interactibles/Level2_Puzzle/Tiles/Tile.Tile_C|GetNeighbours _currenttile))
  (bind _value (Utilities|Map|Find _neighbours "/Game/Blueprints/Interactibles/Level2_Puzzle/Base/Left.Left"))
  (if (Variables|Default|GetCanMoveOverride)
    (Utilities|IsValid (Variables|Default|GetTargetTile)
      (:Is%20Not%20Valid
        (Utilities|IsValid _value
          (:Is%20Valid
            (CallFunction|MovetoTile _value)
            (CallFunction|RotatetoDirection "/Game/Blueprints/Interactibles/Level2_Puzzle/Base/Left.Left")))))))

(event EventBeginPlay
  (bind _self self)
  (bind _outactors (Actor|GetAllActorsOfClass "/Game/Blueprints/Interactibles/Level2_Puzzle/PressurePlates/PressurePlateBP.PressurePlateBP_C"))
  (bind _output_get (Variables|Default|SetPressurePlates _outactors))
  (for _array_element _output_get
    (Variables|/Game/Blueprints/Interactibles/Level2_Puzzle/PressurePlates/PressurePlateBP.PressurePlateBP_C|SetBoulderBP _array_element _self)
    (Development|PrintString (Utilities|GetDisplayName _array_element))
    (Variables|/Game/Blueprints/Interactibles/Level2_Puzzle/PressurePlates/PressurePlateBP.PressurePlateBP_C|SetBoulderIn _array_element true)
    (Development|PrintString (Utilities|String|ToString(Boolean) (Variables|Default|GetCanMoveOverride))))
  (bind _asthird_person_character (Utilities|Casting|CastToThirdPersonCharacter (Game|GetPlayerCharacter 0)))
  (Variables|/Game/ThirdPersonBP/Blueprints/ThirdPersonCharacter.ThirdPersonCharacter_C|SetBoulder _asthird_person_character _self))

(event Collision|EventActorBeginOverlap
  (params (OtherActor :type Actor%20Object%20Reference)))

(event EventTick
  (params (DeltaSeconds :type Float%20%28single-precision%29)))

(fn ConstructionScript)