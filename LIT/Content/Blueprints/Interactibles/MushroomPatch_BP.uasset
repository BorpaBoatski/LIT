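; MushroomPatch_BP is a scavengeable mushroom patch that the player picks once through a light interact event.
; Picking sets the third-person character's MushroomCount, passes the item to ReceiveItem, clears Scavengable and plays a pickup sound.
; Once it is no longer scavengeable, Tick plays the LightOff timeline, which drives the emissive strength of a dynamic material created in the construction script.
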(event EventLightInteractReceive
  (params (LightProjectile :type Light%20Projectile%20Object%20Reference))
  ;[1 1 1] Pick
  (if (Variables|Default|GetScavengable)
    (bind _asthird_person_character (Utilities|Casting|CastToThirdPersonCharacter (Game|GetPlayerCharacter 0)))
    (Variables|/Game/ThirdPersonBP/Blueprints/ThirdPersonCharacter.ThirdPersonCharacter_C|SetMushroomCount _asthird_person_character 1)
    (Default|ReceiveItem _asthird_person_character 4)
    (Variables|Default|SetScavengable false)
    (Audio|PlaySoundatLocation "/Game/Audio/SFX/Interactibles/Audio_Item_Pickup_Cue.Audio_Item_Pickup_Cue" (Transformation|GetActorLocation))))

(event EventTick
  (params (DeltaSeconds :type Float%20%28single-precision%29))
  ;[1 1 1] Change emissive
  (if (not (Variables|Default|GetScavengable))
    (bind _emissive_strength (Timeline|LightOff Play)
      (:Update
        (Rendering|Material|SetScalarParameterValue (Variables|Default|GetMaterial) "Emmissive strength" _emissive_strength :!class /Script/Engine.MaterialInstanceDynamic)))))

(fn ConstructionScript
  (bind _returnvalue (Rendering|Material|CreateDynamicMaterialInstance (Variables|Default|GetStaticMesh) 0 0 :!class /Script/Engine.PrimitiveComponent))
  (Variables|Default|SetMaterial _returnvalue))