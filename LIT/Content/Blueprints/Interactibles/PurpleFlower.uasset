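; PurpleFlower is an interactible that awards the player a berry when a LightProjectile hits it.
; On Box overlap, if Scavengable is set, it casts the other actor to LightProjectile and increments BerryCount on the player's ThirdPersonCharacter.
; It then flags HasPurpFlowerInteracted on TutorialText when that reference is valid.
; The graph never clears Scavengable or removes the flower.
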(event OnComponentBeginOverlap(Box)
  (params (OverlappedComponent :type Primitive%20Component%20Object%20Reference) (OtherActor :type Actor%20Object%20Reference) (OtherComp :type Primitive%20Component%20Object%20Reference) (OtherBodyIndex :type Integer) (bFromSweep :type Boolean) (SweepResult :type Hit%20Result%20Structure%20%28by%20ref%29))
  (if (Variables|Default|GetScavengable)
    (Utilities|Casting|CastToLightProjectile OtherActor)
    (bind _asthird_person_character (Utilities|Casting|CastToThirdPersonCharacter (Game|GetPlayerCharacter 0)))
    (Math|Integer|IncrementInt (Variables|/Game/ThirdPersonBP/Blueprints/ThirdPersonCharacter.ThirdPersonCharacter_C|GetBerryCount _asthird_person_character)
      (:%20%20
        (Utilities|IsValid (Variables|Default|GetTutorialText)
          (:Is%20Valid
            (Variables|/Game/Blueprints/Placeholder/TutorialTextRender.TutorialTextRender_C|SetHasPurpFlowerInteracted (Variables|Default|GetTutorialText) true)))))))

(fn ConstructionScript)