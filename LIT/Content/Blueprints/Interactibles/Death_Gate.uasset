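; Death gate trap that kills an SK_01 character with moving spikes once two pillars are lit by light projectiles.
; Each pillar hit destroys the projectile and lights its pulse; both together enable spike overlaps and trigger the spike movement, then everything resets.
; A charging SK_01 hitting the vines starts struggling and arms KillOn, so a spike overlap sets it and its animation instance dead.
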(event OnComponentBeginOverlap(Pillar2Box)
  (params (OverlappedComponent :type Primitive%20Component%20Object%20Reference) (OtherActor :type Actor%20Object%20Reference) (OtherComp :type Primitive%20Component%20Object%20Reference) (OtherBodyIndex :type Integer) (bFromSweep :type Boolean) (SweepResult :type Hit%20Result%20Structure%20%28by%20ref%29))
  ;[1 1 1] Pillar 2
  (bind _aslight_projectile (Utilities|Casting|CastToLightProjectile OtherActor))
  (Actor|DestroyActor _aslight_projectile)
  (if (not (Variables|Default|GetReset))
    (bind _output_get (Variables|Default|SetPillarSwitch2 true))
    (Rendering|Material|SetMaterial (Variables|Default|GetPulse2) 0 "/Game/Materials/LightBall_Inst.LightBall_Inst")
    (CallFunction|ActivateGate (Variables|Default|GetPillarSwitch1) _output_get)
    (Development|PrintString "DeathGate : Pillar 2")))

(event OnComponentHit(Vines)
  (params (HitComponent :type Primitive%20Component%20Object%20Reference) (OtherActor :type Actor%20Object%20Reference) (OtherComp :type Primitive%20Component%20Object%20Reference) (NormalImpulse :type Vector :default "0, 0, 0") (Hit :type Hit%20Result%20Structure%20%28by%20ref%29))
  ;[1 1 1] Vines
  (bind _assk_01 (Utilities|Casting|CastToSK_01 OtherActor))
  (Collision|SetCollisionResponsetoChannel (Variables|/Script/Engine.Character|GetCapsuleComponent _assk_01) "ECC_GameTraceChannel1" "ECR_Ignore")
  (if (ScalableFloat|GetValueasBool (AI|GetBlackboard _assk_01) (Variables|Default|GetCharge))
    (Variables|/Game/Blueprints/AI/Shrine_Keeper_01/SK_01.SK_01_C|SetDelay _assk_01 (Variables|Default|GetDelayReset))
    (bind _asanim_sk01_new (Utilities|Casting|CastToAnim_SK01_New (Components|SkeletalMesh|GetAnimInstance (Variables|/Script/Engine.Character|GetMesh _assk_01))))
    (Variables|/Game/Models_Animations/ShrineKeeper_01/Anim_SK01_New.Anim_SK01_New_C|SetisStruggle _asanim_sk01_new true)
    (Variables|Default|SetKillOn true)))

(event OnComponentBeginOverlap(Spikes)
  (params (OverlappedComponent :type Primitive%20Component%20Object%20Reference) (OtherActor :type Actor%20Object%20Reference) (OtherComp :type Primitive%20Component%20Object%20Reference) (OtherBodyIndex :type Integer) (bFromSweep :type Boolean) (SweepResult :type Hit%20Result%20Structure%20%28by%20ref%29))
  ;[1 1 1] Kill SK
  (bind _assk_01 (Utilities|Casting|CastToSK_01 OtherActor))
  (if (Variables|Default|GetKillOn)
    (Variables|/Game/Blueprints/AI/Shrine_Keeper_01/SK_01.SK_01_C|SetisDead _assk_01 true)
    (bind _asanim_sk01_new (Utilities|Casting|CastToAnim_SK01_New (Components|SkeletalMesh|GetAnimInstance (Variables|/Script/Engine.Character|GetMesh _assk_01))))
    (Variables|/Game/Models_Animations/ShrineKeeper_01/Anim_SK01_New.Anim_SK01_New_C|SetisDead _asanim_sk01_new true)
    (Variables|Default|SetKillOn false)))

(event OnComponentBeginOverlap(Pillar1Box)
  (params (OverlappedComponent :type Primitive%20Component%20Object%20Reference) (OtherActor :type Actor%20Object%20Reference) (OtherComp :type Primitive%20Component%20Object%20Reference) (OtherBodyIndex :type Integer) (bFromSweep :type Boolean) (SweepResult :type Hit%20Result%20Structure%20%28by%20ref%29))
  ;[1 1 1] Pillar 1
  (bind _aslight_projectile (Utilities|Casting|CastToLightProjectile OtherActor))
  (Actor|DestroyActor _aslight_projectile)
  (if (not (Variables|Default|GetReset))
    (bind _output_get (Variables|Default|SetPillarSwitch1 true))
    (Rendering|Material|SetMaterial (Variables|Default|GetPulse1) 0 "/Game/Materials/LightBall_Inst.LightBall_Inst")
    (CallFunction|ActivateGate _output_get (Variables|Default|GetPillarSwitch2))
    (Development|PrintString "DeathGate : Pillar 1")))

(event Custom|MoveGate
  (bind _spikes (Variables|Default|GetSpikes))
  (bind _relativelocation (Variables|/Script/Engine.SceneComponent|GetRelativeLocation _spikes))
  ;[1 1 1] Gate Movement
  (Development|PrintString "DeathGate : Move Spikes" false)
  (Components|MoveComponentTo _spikes (+ _relativelocation "0, 0,13000.000000") "0, 0, 0" false false 0.2 false)
  (Variables|Default|SetReset true)
  (Components|MoveComponentTo _spikes (- _relativelocation "0, 0,13000.000000") "0, 0, 0" false false 3.0 false)
  (Variables|Default|SetPillarSwitch1 false)
  (Variables|Default|SetPillarSwitch2 false)
  (Variables|Default|SetReset false)
  (Variables|/Script/Engine.PrimitiveComponent|SetbGenerateOverlapEvents (Variables|Default|GetSpikes) false)
  (Rendering|Material|SetMaterial (Variables|Default|GetPulse1) 0 "/Game/Materials/Pulse_M_Inst.Pulse_M_Inst")
  (Rendering|Material|SetMaterial (Variables|Default|GetPulse2) 0 "/Game/Materials/Pulse_M_Inst.Pulse_M_Inst"))

(fn ConstructionScript)

(fn ActivateGate
  (params (Switch1 :type Boolean) (Switch2 :type Boolean))
  (if (and Switch1 Switch2)
    (Variables|/Script/Engine.PrimitiveComponent|SetbGenerateOverlapEvents (Variables|Default|GetSpikes) true)
    (CallFunction|MoveGate)))