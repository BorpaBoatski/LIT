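; Checkpoint interactible that records the player's progress and respawn point when its box trigger is overlapped.
; It loads the CharacterData_BP save from the slot named in GameInstance_BP, then passes it the player character's health, item and ability flags, and current transform through SetData.
; The stored level is carried over unchanged, and a debug message reports the save.
; The overlapping actor is not checked, and any disk write is left to SetData.
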(event OnComponentBeginOverlap(Box)
  (params (OverlappedComponent :type Primitive%20Component%20Object%20Reference) (OtherActor :type Actor%20Object%20Reference) (OtherComp :type Primitive%20Component%20Object%20Reference) (OtherBodyIndex :type Integer) (bFromSweep :type Boolean) (SweepResult :type Hit%20Result%20Structure%20%28by%20ref%29))
  (bind _asgame_instance_bp (Utilities|Casting|CastToGameInstance_BP (Game|GetGameInstance)))
  (bind _returnvalue (SaveGame|LoadGamefromSlot (Variables|/Game/Blueprints/SaveGames/GameInstance_BP.GameInstance_BP_C|GetCharacterDataName _asgame_instance_bp)))
  (bind _ascharacter_data_bp (Utilities|Casting|CastToCharacterData_BP _returnvalue))
  (bind _asthird_person_character (Utilities|Casting|CastToThirdPersonCharacter (Game|GetPlayerCharacter 0)))
  (Default|SetData _ascharacter_data_bp (Utilities|Struct|MakeS_MainCharacter (Variables|/Game/ThirdPersonBP/Blueprints/ThirdPersonCharacter.ThirdPersonCharacter_C|GetHealth _asthird_person_character) (Variables|/Game/ThirdPersonBP/Blueprints/ThirdPersonCharacter.ThirdPersonCharacter_C|GethasBerry _asthird_person_character) (Variables|/Game/ThirdPersonBP/Blueprints/ThirdPersonCharacter.ThirdPersonCharacter_C|GethasMushroom _asthird_person_character) (Variables|/Game/ThirdPersonBP/Blueprints/ThirdPersonCharacter.ThirdPersonCharacter_C|GethasCicada _asthird_person_character) (Variables|/Game/ThirdPersonBP/Blueprints/ThirdPersonCharacter.ThirdPersonCharacter_C|GethasIronBody _asthird_person_character) (Variables|/Game/ThirdPersonBP/Blueprints/ThirdPersonCharacter.ThirdPersonCharacter_C|GethasPowder _asthird_person_character) (.S_Level (Utilities|Struct|BreakS_MainCharacter (Variables|/Game/Blueprints/SaveGames/CharacterData_BP.CharacterData_BP_C|GetCharacterData _ascharacter_data_bp))) (Transformation|GetActorTransform _asthird_person_character)))
  (Development|PrintString "Checkpoint : Saved"))

(fn ConstructionScript)