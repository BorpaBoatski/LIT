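; PiranhaShoot is a hazard that repeatedly launches along its forward vector and damages the player on contact.
; The construction script feeds exposed speed and gravity values into a ProjectileMovement component.
; A looping timer runs ZCheck, which resets the actor to its stored start location and relaunches it once the mesh is at or below that height.
; Each launch re-arms damage, so a mesh overlap hurts ThirdPersonCharacter only once per launch.
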(event OnComponentBeginOverlap(SkeletalMesh)
  (params (OverlappedComponent :type Primitive%20Component%20Object%20Reference) (OtherActor :type Actor%20Object%20Reference) (OtherComp :type Primitive%20Component%20Object%20Reference) (OtherBodyIndex :type Integer) (bFromSweep :type Boolean) (SweepResult :type Hit%20Result%20Structure%20%28by%20ref%29))
  (if (Variables|Default|GetCanDamage)
    (bind _asthird_person_character (Utilities|Casting|CastToThirdPersonCharacter OtherActor))
    (Default|NewPlayerHealthManager _asthird_person_character -1.0)
    (Variables|Default|SetCanDamage false)))

(event EventBeginPlay
  (Variables|Default|SetZLoc (Transformation|GetWorldLocation (Variables|Default|GetSkeletalMesh)))
  (Utilities|Time|SetTimerbyFunctionName 0 "ZCheck" 0.5 true))

(fn ConstructionScript
  (bind _projectilemovement (Variables|Default|GetProjectileMovement))
  (Variables|/Script/Engine.ProjectileMovementComponent|SetProjectileGravityScale _projectilemovement (Variables|Default|GetGravityScale))
  (Variables|/Script/Engine.ProjectileMovementComponent|SetMaxSpeed _projectilemovement (Variables|Default|GetSpeed))
  (Variables|/Script/Engine.ProjectileMovementComponent|SetInitialSpeed _projectilemovement (Variables|Default|GetSpeed)))

(fn ZCheck
  (if (<= (.Z (Math|Vector|BreakVector (Transformation|GetWorldLocation (Variables|Default|GetSkeletalMesh)))) (.Z (Math|Vector|BreakVector (Variables|Default|GetZLoc))))
    (Transformation|SetActorLocation (Variables|Default|GetZLoc) false false)
    (Variables|/Script/Engine.MovementComponent|SetVelocity (Variables|Default|GetProjectileMovement) (* (Transformation|GetActorForwardVector) (Variables|Default|GetSpeed)))
    (Variables|Default|SetCanDamage true)))