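; 4thTabletHolder2 is an interactible holder that releases the fourth tablet for the player to collect.
; Light interactions increment a shot counter; once it reaches two, the next one hides three spheres, moves Top and raises Tablet over time, and makes the tablet pickable.
; A Player-tagged overlap on Collision then sets the 4thTablet flag on ThirdPersonCharacter and destroys the Tablet component.
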(event OnComponentBeginOverlap(Collision)
  (params (OverlappedComponent :type Primitive%20Component%20Object%20Reference) (OtherActor :type Actor%20Object%20Reference) (OtherComp :type Primitive%20Component%20Object%20Reference) (OtherBodyIndex :type Integer) (bFromSweep :type Boolean) (SweepResult :type Hit%20Result%20Structure%20%28by%20ref%29))
  (if (Actor|ActorHasTag OtherActor "Player")
    (if (Variables|Default|GetCanBePicked)
      (bind _asthird_person_character (Utilities|Casting|CastToThirdPersonCharacter OtherActor))
      (Variables|/Game/ThirdPersonBP/Blueprints/ThirdPersonCharacter.ThirdPersonCharacter_C|Set4thTablet _asthird_person_character true)
      (Components|DestroyComponent (Variables|Default|GetTablet)))))

(event EventBeginPlay)

(event Collision|EventActorBeginOverlap
  (params (OtherActor :type Actor%20Object%20Reference))
  (|CallParentFunction OtherActor) ; This node is disabled and will not be called.\nDrag off pins to build functionality.
)

(event EventTick
  (params (DeltaSeconds :type Float%20%28single-precision%29)))

(event EventLightInteractReceive
  (params (LightProjectile :type Light%20Projectile%20Object%20Reference))
  (if (>= (Variables|Default|GetShotCount) 2)
    (Rendering|SetVisibility (Variables|Default|GetSphere1) false false)
    (Rendering|SetVisibility (Variables|Default|GetSphere2) false false)
    (Rendering|SetVisibility (Variables|Default|GetSphere) false false)
    (Components|MoveComponentTo (Variables|Default|GetTop) (+ "0, 0, 0" "0, 0,25.000000") "0,-90.000000, 0" false false 1.0 false)
    (Components|MoveComponentTo (Variables|Default|GetTablet) (+ "0, 0, 0" "0, 0,140.000000") "0, 0, 0" false false 1.0 false)
    (Variables|Default|SetCanBePicked true)
    (else
      (Variables|Default|SetShotCount (+ (Variables|Default|GetShotCount) 1)))))

(fn ConstructionScript
  (|CallParentFunction))