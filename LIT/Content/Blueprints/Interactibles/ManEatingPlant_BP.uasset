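; Man-eating plant interactible that eats actors coming within its reach.
; Overlaps on DetectionBox and EatingRange fill two food lists; Tick runs the bite cooldown while food is detected and yaws the mesh using the first in-range target.
; Eat damages a ThirdPersonCharacter, hides it with input disabled, teleports it to Stomach, then spits it out at Spit after a delay.
; Other actors are destroyed.
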(event OnComponentEndOverlap(Eatingrange)
  (params (OverlappedComponent :type Primitive%20Component%20Object%20Reference) (OtherActor :type Actor%20Object%20Reference) (OtherComp :type Primitive%20Component%20Object%20Reference) (OtherBodyIndex :type Integer))
  ;[1 1 1] Eat Exit
  (Utilities|Array|RemoveItem (Variables|Default|GetInRangeFood) OtherActor))

(event OnComponentBeginOverlap(DetectionBox)
  (params (OverlappedComponent :type Primitive%20Component%20Object%20Reference) (OtherActor :type Actor%20Object%20Reference) (OtherComp :type Primitive%20Component%20Object%20Reference) (OtherBodyIndex :type Integer) (bFromSweep :type Boolean) (SweepResult :type Hit%20Result%20Structure%20%28by%20ref%29))
  ;[1 1 1] Detection Enter
  (Utilities|Array|Add (Variables|Default|GetDetectedFood) OtherActor))

(event OnComponentEndOverlap(DetectionBox)
  (params (OverlappedComponent :type Primitive%20Component%20Object%20Reference) (OtherActor :type Actor%20Object%20Reference) (OtherComp :type Primitive%20Component%20Object%20Reference) (OtherBodyIndex :type Integer))
  ;[1 1 1] Detection Exit
  (Utilities|Array|RemoveItem (Variables|Default|GetDetectedFood) OtherActor))

(event OnComponentBeginOverlap(Eatingrange)
  (params (OverlappedComponent :type Primitive%20Component%20Object%20Reference) (OtherActor :type Actor%20Object%20Reference) (OtherComp :type Primitive%20Component%20Object%20Reference) (OtherBodyIndex :type Integer) (bFromSweep :type Boolean) (SweepResult :type Hit%20Result%20Structure%20%28by%20ref%29))
  ;[1 1 1] Eat Enter
  (Utilities|Array|Add (Variables|Default|GetInRangeFood) OtherActor))

(event Custom|Eat
  (bind _inrangefood (Variables|Default|GetInRangeFood))
  (bind _inrangefood_2 (Variables|Default|GetInRangeFood))
  (bind _skeletalmesh (Variables|Default|GetSkeletalMesh))
  (bind _output (Utilities|Array|Get(acopy) _inrangefood))
  (Development|PrintString "ManEater: Eat")
  (bind _asthird_person_character (Utilities|Casting|CastToThirdPersonCharacter _output)
    (:then
      (Default|NewPlayerHealthManager _asthird_person_character -1.0)
      (CallFunction|HidePlayer true _asthird_person_character)
      (Transformation|SetActorLocation _asthird_person_character (Transformation|GetWorldLocation (Variables|Default|GetStomach)) false true)
      (Components|MoveComponentTo _skeletalmesh "0, 0, 0" "0, 0, 0" false false (/ (Variables|Default|GetEatDuration) 2.0) false)
      (Utilities|FlowControl|Delay (/ (Variables|Default|GetEatDuration) 2.0))
      (Transformation|SetActorLocation _asthird_person_character (Transformation|GetWorldLocation (Variables|Default|GetSpit)) false true)
      (CallFunction|HidePlayer false _asthird_person_character))
    (:CastFailed
      (Actor|DestroyActor _output)
      (Components|MoveComponentTo _skeletalmesh "0, 0, 0" "0, 0, 0" false false 2.0 false)))
  (Utilities|Array|RemoveItem (Variables|Default|GetDetectedFood) (Utilities|Array|Get(acopy) _inrangefood_2))
  (Utilities|Array|RemoveIndex _inrangefood_2)
  (Variables|Default|SetCanEatTimer (Variables|Default|GetCanEatCooldown))
  (Variables|Default|SetCanEat true))

(event EventTick
  (params (DeltaSeconds :type Float%20%28single-precision%29))
  (bind _inrangefood (Variables|Default|GetInRangeFood))
  (if (> (Utilities|Array|Length (Variables|Default|GetDetectedFood)) 0)
    (Variables|Default|SetCanEatTimer (- (Variables|Default|GetCanEatTimer) DeltaSeconds))
    (if (> (Utilities|Array|Length _inrangefood) 0)
      (Transformation|SetRelativeRotation (Variables|Default|GetSkeletalMesh) (Math|Rotator|MakeRotator 0.0 0.0 (.Yaw (Math|Rotator|BreakRotator (Math|Rotator|FindLookatRotation (Transformation|GetActorLocation (Utilities|Array|Get(acopy) _inrangefood)) (Transformation|GetActorLocation))))) false false)
      (if (and (<= (Variables|Default|GetCanEatTimer) 0.0) (Math|Boolean|Equal(Boolean) (Variables|Default|GetCanEat) true))
        (Variables|Default|SetCanEat false)
        (CallFunction|Eat)))
    (else
      (Variables|Default|SetCanEatTimer (Variables|Default|GetCanEatCooldown)))))

(fn ConstructionScript)

(fn HidePlayer
  (params (Hide? :type Boolean) (ThirdPerson :type Third%20Person%20Character%20Object%20Reference))
  (if Hide?
    (Rendering|SetActorHiddenInGame ThirdPerson true)
    (Input|DisableInput ThirdPerson (Game|GetPlayerController 0))
    (Collision|SetCollisionResponsetoChannel (Variables|Default|GetSkeletalMesh) "ECC_Camera" "ECR_Ignore")
    (else
      (Rendering|SetActorHiddenInGame ThirdPerson false)
      (Input|EnableInput ThirdPerson (Game|GetPlayerController 0))
      (Collision|SetCollisionResponsetoChannel (Variables|Default|GetSkeletalMesh) "ECC_Camera" "ECR_Block"))))