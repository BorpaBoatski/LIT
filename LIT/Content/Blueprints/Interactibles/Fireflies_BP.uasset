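; Interactive fireflies actor that flees from whatever touches its box trigger, ignoring components tagged Light.
; On overlap it yaws to face away from the other actor, then Tick uses VInterpTo to move it continuously along its forward vector.
; Ending the overlap starts a six-second timer, after which it snaps back to the location saved at BeginPlay and stops moving.
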(event OnComponentBeginOverlap(Box)
  (params (OverlappedComponent :type Primitive%20Component%20Object%20Reference) (OtherActor :type Actor%20Object%20Reference) (OtherComp :type Primitive%20Component%20Object%20Reference) (OtherBodyIndex :type Integer) (bFromSweep :type Boolean) (SweepResult :type Hit%20Result%20Structure%20%28by%20ref%29))
  ;[1 1 1] Rotates Fireflies to face away from whatever object came into contact with it
  (if (not (Components|ComponentHasTag OtherComp "Light"))
    (Transformation|SetActorRotation (Math|Rotator|MakeRotator 0.0 0.0 (+ (.Yaw (Math|Rotator|BreakRotator (Math|Rotator|FindLookatRotation (Transformation|GetActorLocation) (Transformation|GetActorLocation OtherActor)))) 1.8e+02)))
    (Variables|Default|SetIsOverlapping true)))

(event OnComponentEndOverlap(Box)
  (params (OverlappedComponent :type Primitive%20Component%20Object%20Reference) (OtherActor :type Actor%20Object%20Reference) (OtherComp :type Primitive%20Component%20Object%20Reference) (OtherBodyIndex :type Integer))
  ;[1 1 1] Sets the location of fireflies to it's original position after 6 seconds
  (if (not (Components|ComponentHasTag OtherComp "Light"))
    (Utilities|Time|SetTimerbyEvent (delegate Custom|ReturnToOriginalLocation) 6.0)))

(event Custom|ReturnToOriginalLocation
  ;[1 1 1] Sets the location of fireflies to it's original position after 6 seconds
  (Transformation|SetActorLocation (Variables|Default|GetStart_Loc) false false)
  (Variables|Default|SetIsOverlapping false))

(event EventBeginPlay
  ;[1 1 1] Sets starting location of Fireflies
  (Variables|Default|SetStart_Loc (Transformation|GetActorLocation)))

(event EventTick
  (params (DeltaSeconds :type Float%20%28single-precision%29))
  ;[1 1 1] Moves fireflies in forward direction
  (if (Variables|Default|GetIsOverlapping)
    (Transformation|SetActorLocation (Math|Interpolation|VInterpTo (Transformation|GetActorLocation) (+ (Transformation|GetActorLocation) (* (Transformation|GetActorForwardVector) 3e+02)) DeltaSeconds 1.0) false false)))

(fn ConstructionScript)