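; Totem interactible that lights up when struck by a light projectile and flashes goon enemies that come near it.
; Receiving light plays a sound, then shows the point light and enables sphere overlaps for a time scaled by the projectile's charge, ignoring hits while lit.
; Goons beginning overlap receive the flash interface call.
; An older in-range list and line-of-sight trace check remains disconnected.
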(event OnComponentBeginOverlap(Sphere)
  (params (OverlappedComponent :type Primitive%20Component%20Object%20Reference) (OtherActor :type Actor%20Object%20Reference) (OtherComp :type Primitive%20Component%20Object%20Reference) (OtherBodyIndex :type Integer) (bFromSweep :type Boolean) (SweepResult :type Hit%20Result%20Structure%20%28by%20ref%29))
  ;[1 1 1] Light collision
  (bind _asenemy_goon_base (Utilities|Casting|CastToEnemy_Goon_Base OtherActor))
  (Default|FlashInterfaceReceive _asenemy_goon_base OtherActor))

(event OnComponentEndOverlap(Sphere)
  (params (OverlappedComponent :type Primitive%20Component%20Object%20Reference) (OtherActor :type Actor%20Object%20Reference) (OtherComp :type Primitive%20Component%20Object%20Reference) (OtherBodyIndex :type Integer))
  ;[1 1 1] Light collision
)

(event Custom|TraceCheck
  ;[1 1 1] Scare enemy (OLD)
)

(event EventTick
  (params (DeltaSeconds :type Float%20%28single-precision%29))
  ;[1 1 1] Tick
)

(event EventLightInteractReceive
  (params (LightProjectile :type Light%20Projectile%20Object%20Reference))
  (bind _pointlight (Variables|Default|GetPointLight))
  (bind _sphere (Variables|Default|GetSphere))
  ;[1 1 1] Light On & Off
  (Variables|Default|SetDurationTime (* (Variables|/Game/ThirdPersonBP/Blueprints/LightProjectile.LightProjectile_C|GetLightCharge LightProjectile) 3.5))
  (if (not (Rendering|IsVisible _pointlight))
    (Audio|PlaySoundatLocation "/Game/Audio/SFX/Interactibles/totem_lightup_Cue.totem_lightup_Cue" (Transformation|GetActorLocation self))
    (Rendering|ToggleVisibility _pointlight false)
    (Variables|/Script/Engine.PrimitiveComponent|SetbGenerateOverlapEvents _sphere true)
    (Utilities|FlowControl|Delay (Variables|Default|GetDurationTime))
    (Rendering|ToggleVisibility _pointlight false)
    (Variables|Default|SetDurationTime 0.0)
    (Variables|/Script/Engine.PrimitiveComponent|SetbGenerateOverlapEvents _sphere false)
    (Utilities|Array|Clear (Variables|Default|GetInRange))))

(fn ConstructionScript)