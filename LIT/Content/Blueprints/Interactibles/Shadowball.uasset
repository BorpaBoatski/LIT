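; Shadowball is a moving hazard that damages the ThirdPersonCharacter on overlap with its skeletal mesh.
; From BeginPlay it loops two MoveComponentTo calls, adding then subtracting NewDestination from its current location, timed by the length of location minus NewDestination divided by Speed.
; A hit passes -1 to the character's NewPlayerHealthManager, then the DealDamage flag blocks further hits during a 1.5-second retriggerable delay.
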(event OnComponentBeginOverlap(SkeletalMesh)
  (params (OverlappedComponent :type Primitive%20Component%20Object%20Reference) (OtherActor :type Actor%20Object%20Reference) (OtherComp :type Primitive%20Component%20Object%20Reference) (OtherBodyIndex :type Integer) (bFromSweep :type Boolean) (SweepResult :type Hit%20Result%20Structure%20%28by%20ref%29))
  (if (Variables|Default|GetDealDamage)
    (bind _asthird_person_character (Utilities|Casting|CastToThirdPersonCharacter OtherActor))
    (Default|NewPlayerHealthManager _asthird_person_character -1.0)
    (Variables|Default|SetDealDamage false)
    (Utilities|FlowControl|RetriggerableDelay 1.5)
    (Variables|Default|SetDealDamage true)))

(event EventBeginPlay
  (bind _returnvalue (Transformation|GetActorLocation))
  (bind _speed (Variables|Default|GetSpeed))
  (bind _newdestination (Variables|Default|GetNewDestination))
  (bind _returnvalue_2 (- _returnvalue _newdestination))
  (bind _returnvalue_3 (Math|Vector|VectorLength _returnvalue_2))
  (bind _returnvalue_4 (/ _returnvalue_3 _speed))
  (Development|PrintString (Utilities|String|Append "Shadowball: " (Utilities|String|ToString(Float) _returnvalue_4) " travel time"))
  (Components|MoveComponentTo (Variables|Default|GetDefaultSceneRoot) (+ _returnvalue (Variables|Default|GetNewDestination)) "0, 0, 0" false false _returnvalue_4 false :!label _label)
  (Components|MoveComponentTo (Variables|Default|GetDefaultSceneRoot) (- (Transformation|GetActorLocation) (Variables|Default|GetNewDestination)) "0, 0, 0" false false _returnvalue_4 false)
  (goto _label))

(fn ConstructionScript)