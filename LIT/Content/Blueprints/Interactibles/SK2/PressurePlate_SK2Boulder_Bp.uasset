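; Pressure plate Blueprint that spawns a BoulderSK2_BP at BoulderSpawnTransform when a Player-tagged actor steps on it.
; Box overlap events set a ReleaseBoulder flag, which a fast looping timer polls to spawn when off cooldown.
; A second looping timer clears the cooldown after a BoulderCooldown delay.
; Spawning clears the flag, so staying on the plate does not retrigger it.
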(event OnComponentBeginOverlap(Box)
  (params (OverlappedComponent :type Primitive%20Component%20Object%20Reference) (OtherActor :type Actor%20Object%20Reference) (OtherComp :type Primitive%20Component%20Object%20Reference) (OtherBodyIndex :type Integer) (bFromSweep :type Boolean) (SweepResult :type Hit%20Result%20Structure%20%28by%20ref%29))
  ;[1 1 1] If player comes into contact with pressure plate, set release boulder to true
  (if (Actor|ActorHasTag OtherActor "Player")
    (Variables|Default|SetReleaseBoulder true)))

(event OnComponentEndOverlap(Box)
  (params (OverlappedComponent :type Primitive%20Component%20Object%20Reference) (OtherActor :type Actor%20Object%20Reference) (OtherComp :type Primitive%20Component%20Object%20Reference) (OtherBodyIndex :type Integer))
  ;[1 1 1] If player leaves pressure plate, set release boulder to false
  (if (Actor|ActorHasTag OtherActor "Player")
    (Variables|Default|SetReleaseBoulder false)))

(event Custom|Tick1
  ;[1 1 1] Release a boulder if not on cooldown and if player is on pressure plate
  (if (Variables|Default|GetReleaseBoulder)
    (if (not (Variables|Default|GetOnCooldown))
      (Variables|Default|SetReleaseBoulder false)
      (Variables|Default|SetOnCooldown true)
      (Game|SpawnActorfromClass "/Game/Blueprints/Interactibles/SK2/BoulderSK2_Bp.BoulderSK2_BP_C" (Transformation|GetWorldTransform (Variables|Default|GetBoulderSpawnTransform)) "Undefined" 0 0))))

(event Custom|Tick2
  ;[1 1 1] Resets boulder cooldown after duration
  (if (Variables|Default|GetOnCooldown)
    (Utilities|FlowControl|Delay (Variables|Default|GetBoulderCooldown))
    (Variables|Default|SetOnCooldown false)))

(event EventBeginPlay
  ;[1 1 1] Run tick functions continuously
  (Utilities|Time|SetTimerbyFunctionName 0 "Tick1" 0.01 true)
  (Utilities|Time|SetTimerbyFunctionName 0 "Tick2" 0.01 true))

(fn ConstructionScript)