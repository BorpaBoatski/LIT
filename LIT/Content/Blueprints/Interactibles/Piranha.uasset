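; Piranha is an interactible hazard that spins continuously and damages the player on touch.
; On BeginPlay it sets the RotatingMovement pitch rate from SpinRate.
; When the Cube begins overlapping a ThirdPersonCharacter, it passes -1 to that character's NewPlayerHealthManager.
; An unconnected node that would offset the Cube vertically by Distance never runs.
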(event OnComponentBeginOverlap(Cube)
  (params (OverlappedComponent :type Primitive%20Component%20Object%20Reference) (OtherActor :type Actor%20Object%20Reference) (OtherComp :type Primitive%20Component%20Object%20Reference) (OtherBodyIndex :type Integer) (bFromSweep :type Boolean) (SweepResult :type Hit%20Result%20Structure%20%28by%20ref%29))
  (bind _asthird_person_character (Utilities|Casting|CastToThirdPersonCharacter OtherActor))
  (Default|NewPlayerHealthManager _asthird_person_character -1.0))

(event EventBeginPlay
  (Variables|/Script/Engine.RotatingMovementComponent|SetRotationRate (Variables|Default|GetRotatingMovement) (Math|Rotator|MakeRotator 0.0 (Variables|Default|GetSpinRate) 0.0)))

(fn ConstructionScript)