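; Game instance that applies the saved audio options when the game starts.
; After a short delay, Init pushes a global sound mix, loads the options save object and applies Master, SFX, Ambience and Music volumes.
; SetVolume clamps each value, overrides the matching sound class in the mix and passes it back through SetOptions.
; LoadOptions reads the save slot, creating a new options object when none exists.
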(event EventInit
  (bind _saveoptions (Variables|Default|GetSaveOptions))
  (bind _s_options (Variables|/Game/Blueprints/SaveGames/SaveOptions_BP.SaveOptions_BP_C|GetS_Options _saveoptions))
  (bind (_mastervolume _sfxvolume _ambiencevolume _musicvolume) (Utilities|Struct|BreakS_Options _s_options))
  (Utilities|FlowControl|Delay 0.2) ; needed or else functions won't work
  ;[1 1 1] Set Sound Mixes
  (Class|GameplayStatics|SetBaseSoundMix "/Game/Blueprints/Audio/SM_Global.SM_Global")
  (Audio|PushSoundMixModifier "/Game/Blueprints/Audio/SM_Global.SM_Global")
  ;[1 1 1] Load and Set Volume levels
  (Variables|Default|GetSaveOptions
    (:then
      _)
    (:else
      (CallFunction|LoadOptions)))
  (Utilities|FlowControl|Sequence
    (:then_0
      (CallFunction|SetVolume "NewEnumerator0" _mastervolume))
    (:then_1
      (CallFunction|SetVolume "NewEnumerator1" _sfxvolume))
    (:then_2
      (CallFunction|SetVolume "NewEnumerator2" _ambiencevolume))
    (:then_3
      (CallFunction|SetVolume "NewEnumerator3" _musicvolume))))

(fn SetVolume
  (params (E_SoundChannel :type E_SoundChannel%20Enum :default "NewEnumerator0") (Value :type Float%20%28single-precision%29))
  (bind _returnvalue (Math|Float|Clamp(Float) Value))
  (Variables|Default|GetSaveOptions
    (:then
      _)
    (:else
      (CallFunction|LoadOptions)))
  (switch Utilities|FlowControl|Switch|SwitchonE_SoundChannel E_SoundChannel
    (:NewEnumerator0
      ;[1 1 1] Set Master Volume
      (Audio|SetSoundMixClassOverride "/Game/Blueprints/Audio/SM_Global.SM_Global" "/Game/Blueprints/Audio/SC_Master.SC_Master" _returnvalue 1.0 1.0 true)
      (bind _structout (Utilities|Struct|SetmembersinS_Options (Variables|/Game/Blueprints/SaveGames/SaveOptions_BP.SaveOptions_BP_C|GetS_Options (Variables|Default|GetSaveOptions)) _returnvalue))
      (Default|SetOptions (Variables|Default|GetSaveOptions) _structout))
    (:NewEnumerator1
      ;[1 1 1] Set SFX Volume
      (Audio|SetSoundMixClassOverride "/Game/Blueprints/Audio/SM_Global.SM_Global" "/Game/Blueprints/Audio/SC_SFX.SC_SFX" _returnvalue 1.0 1.0 true)
      (bind _structout_2 (Utilities|Struct|SetmembersinS_Options (Variables|/Game/Blueprints/SaveGames/SaveOptions_BP.SaveOptions_BP_C|GetS_Options (Variables|Default|GetSaveOptions)) _returnvalue))
      (Default|SetOptions (Variables|Default|GetSaveOptions) _structout_2))
    (:NewEnumerator2
      ;[1 1 1] Set Ambience Volume
      (Audio|SetSoundMixClassOverride "/Game/Blueprints/Audio/SM_Global.SM_Global" "/Game/Blueprints/Audio/SC_Ambience.SC_Ambience" _returnvalue 1.0 1.0 true)
      (bind _structout_3 (Utilities|Struct|SetmembersinS_Options (Variables|/Game/Blueprints/SaveGames/SaveOptions_BP.SaveOptions_BP_C|GetS_Options (Variables|Default|GetSaveOptions)) _returnvalue))
      (Default|SetOptions (Variables|Default|GetSaveOptions) _structout_3))
    (:NewEnumerator3
      ;[1 1 1] Set Music Volume
      (Audio|SetSoundMixClassOverride "/Game/Blueprints/Audio/SM_Global.SM_Global" "/Game/Blueprints/Audio/SC_Music.SC_Music" _returnvalue 1.0 1.0 true)
      (bind _structout_4 (Utilities|Struct|SetmembersinS_Options (Variables|/Game/Blueprints/SaveGames/SaveOptions_BP.SaveOptions_BP_C|GetS_Options (Variables|Default|GetSaveOptions)) _returnvalue))
      (Default|SetOptions (Variables|Default|GetSaveOptions) _structout_4))))

(fn LoadOptions
  (bind _returnvalue (SaveGame|DoesSaveGameExist (Variables|Default|GetSaveOptionsName)))
  (if _returnvalue
    _
    (else
      (Variables|Default|GetSaveOptions
        (:then
          _)
        (:else
          (bind _returnvalue_2 (SaveGame|CreateSaveGameObject "/Game/Blueprints/SaveGames/SaveOptions_BP.SaveOptions_BP_C"))
          (Variables|Default|SetSaveOptions _returnvalue_2)))))
  (bind _returnvalue_3 (SaveGame|LoadGamefromSlot (Variables|Default|GetSaveOptionsName)))
  (bind _assave_options_bp (Utilities|Casting|CastToSaveOptions_BP _returnvalue_3))
  (Variables|Default|SetSaveOptions _assave_options_bp))