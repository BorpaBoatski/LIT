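; DialoguePopUp_BP is a trigger-box actor that shows a two-part tutorial text popup.
; Any begin overlap creates a TotemTutorial widget with MyText, then swaps to MyText2 after a configurable delay and sets HasDisplayed, blocking repeats.
; The widget is removed when a ThirdPersonCharacter leaves the box, or by a five-second delay run from Tick once HasDisplayed is set.
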(event OnComponentEndOverlap(Box)
  (params (OverlappedComponent :type Primitive%20Component%20Object%20Reference) (OtherActor :type Actor%20Object%20Reference) (OtherComp :type Primitive%20Component%20Object%20Reference) (OtherBodyIndex :type Integer))
  ;[1 1 1] Gets rid of text after exiting trigger box
  (Utilities|Casting|CastToThirdPersonCharacter OtherActor)
  (Utilities|IsValid (Variables|Default|GetTotemTutorialWidget)
    (:Is%20Valid
      (Widget|RemovefromParent (Variables|Default|GetTotemTutorialWidget))
      (Variables|Default|SetTotemTutorialWidget 0))))

(event OnComponentBeginOverlap(Box)
  (params (OverlappedComponent :type Primitive%20Component%20Object%20Reference) (OtherActor :type Actor%20Object%20Reference) (OtherComp :type Primitive%20Component%20Object%20Reference) (OtherBodyIndex :type Integer) (bFromSweep :type Boolean) (SweepResult :type Hit%20Result%20Structure%20%28by%20ref%29))
  ;[1 1 1] Spawns text when trigger box is entered,
  (if (not (Variables|Default|GetHasDisplayed))
    (Utilities|IsValid (Variables|Default|GetTotemTutorialWidget)
      (:Is%20Not%20Valid
        (bind _returnvalue (UserInterface|CreateWidget "/Game/UI/Widgets/TotemTutorial.TotemTutorial_C" (Game|GetPlayerController 0)))
        (bind _output_get (Variables|Default|SetTotemTutorialWidget _returnvalue))
        (UserInterface|Viewport|AddtoViewport _output_get 0)
        (Variables|/Game/UI/Widgets/TotemTutorial.TotemTutorial_C|SetTotemTutorialText (Variables|Default|GetTotemTutorialWidget) (Variables|Default|GetMyText))
        (Utilities|FlowControl|Delay (Variables|Default|GetDelay))
        (Utilities|IsValid (Variables|Default|GetTotemTutorialWidget)
          (:Is%20Valid
            (Variables|/Game/UI/Widgets/TotemTutorial.TotemTutorial_C|SetTotemTutorialText (Variables|Default|GetTotemTutorialWidget) (Variables|Default|GetMyText2))
            (Variables|Default|SetHasDisplayed true)))))))

(event EventTick
  (params (DeltaSeconds :type Float%20%28single-precision%29))
  ;[1 1 1] Gets rid of text after delay
  (if (Variables|Default|GetHasDisplayed)
    (Utilities|FlowControl|Delay 5.0)
    (Utilities|IsValid (Variables|Default|GetTotemTutorialWidget)
      (:Is%20Valid
        (Widget|RemovefromParent (Variables|Default|GetTotemTutorialWidget))
        (Variables|Default|SetTotemTutorialWidget 0)))))

(fn ConstructionScript)