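; Level 1 tutorial NPC (Sifu) that talks the player through Cicada, Mushroom and Iron Body item lessons in sequence.
; BeginPlay gathers Dialogue table rows by NPC ID; Interact advances lines in a widget, closed on leaving the trigger box.
; Interact also drops each lesson's item and, once looping timers detect pickup and use, unlocks the next stage, teleporting after the first two.
; A separate event fires a light projectile for a cutscene.
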(event OnComponentEndOverlap(Box)
  (params (OverlappedComponent :type Primitive%20Component%20Object%20Reference) (OtherActor :type Actor%20Object%20Reference) (OtherComp :type Primitive%20Component%20Object%20Reference) (OtherBodyIndex :type Integer))
  ;[1 1 1] After exiting collision box/trigger box dialogue window will disappear
  (Utilities|Casting|CastToThirdPersonCharacter OtherActor)
  (Utilities|IsValid (Variables|Default|GetDialogueWidget)
    (:Is%20Valid
      (Widget|RemovefromParent (Variables|Default|GetDialogueWidget))
      (Variables|Default|SetDialogueWidget 0)
      (Variables|Default|SetLineCurrent 0))))

(event Custom|CheckUsedMushroom
  ;[1 1 1] Mushroom Tutorial
  ;;[1 1 1] Check if player used Mushroom
  (if (Variables|Default|GetReachedMushroomTutorial)
    (if (Variables|Default|GetCheckMushroomUsed)
      (bind _asthird_person_character (Utilities|Casting|CastToThirdPersonCharacter (Game|GetPlayerCharacter 0)))
      (if (not (Variables|/Game/ThirdPersonBP/Blueprints/ThirdPersonCharacter.ThirdPersonCharacter_C|GethasMushroom _asthird_person_character))
        (Variables|Default|SetUsedMushroom true)))))

(event Custom|CheckHasCicada
  ;[1 1 1] Cicada Tutorial
  ;;[1 1 1] Check if player picked up Cicada
  (if (Variables|Default|GetStartCheckingCicada)
    (if (Variables|Default|GetReachedCicadaTutorial)
      (bind _asthird_person_character (Utilities|Casting|CastToThirdPersonCharacter (Game|GetPlayerCharacter 0)))
      (if (Variables|/Game/ThirdPersonBP/Blueprints/ThirdPersonCharacter.ThirdPersonCharacter_C|GethasCicada _asthird_person_character)
        (Variables|Default|SetCheckCicadaUsed true)
        (Rendering|SetActorHiddenInGame (Variables|Default|GetE) false)))))

(event Custom|CheckUsedCicada
  ;[1 1 1] Cicada Tutorial
  ;;[1 1 1] Check if player has used Cicada
  (if (Variables|Default|GetReachedCicadaTutorial)
    (if (Variables|Default|GetCheckCicadaUsed)
      (bind _asthird_person_character (Utilities|Casting|CastToThirdPersonCharacter (Game|GetPlayerCharacter 0)))
      (if (not (Variables|/Game/ThirdPersonBP/Blueprints/ThirdPersonCharacter.ThirdPersonCharacter_C|GethasCicada _asthird_person_character))
        (Variables|Default|SetUsedCicada true)))))

(event Custom|CheckUsedIronBody
  ;[1 1 1] Iron Body Tutorial
  ;;[1 1 1] Check if player has used Iron Body
  (if (Variables|Default|GetReachedIronBodyTutorial)
    (if (Variables|Default|GetCheckIronBodyUsed)
      (bind _asthird_person_character (Utilities|Casting|CastToThirdPersonCharacter (Game|GetPlayerCharacter 0)))
      (if (not (Variables|/Game/ThirdPersonBP/Blueprints/ThirdPersonCharacter.ThirdPersonCharacter_C|GethasIronBody _asthird_person_character))
        (Variables|Default|SetUsedIronBody true)))))

(event Custom|Shoot_Lightball_Sifu
  ;[1 1 1] Make sifu shoot out light ball to during cutscene
  (bind _returnvalue (Game|SpawnActorfromClass "/Game/ThirdPersonBP/Blueprints/LightProjectile.LightProjectile_C" (Transformation|GetWorldTransform (Variables|Default|GetArrow1)) "Undefined" 0 0))
  (Variables|/Game/ThirdPersonBP/Blueprints/LightProjectile.LightProjectile_C|SetSunflowerPower _returnvalue true))

(event Custom|CheckHasIronBody
  ;[1 1 1] Iron Body Tutorial
  ;;[1 1 1] Check if player picked up Iron Body
  (if (Variables|Default|GetStartCheckingIronBody)
    (if (Variables|Default|GetReachedIronBodyTutorial)
      (bind _asthird_person_character (Utilities|Casting|CastToThirdPersonCharacter (Game|GetPlayerCharacter 0)))
      (if (Variables|/Game/ThirdPersonBP/Blueprints/ThirdPersonCharacter.ThirdPersonCharacter_C|GethasIronBody _asthird_person_character)
        (Variables|Default|SetCheckIronBodyUsed true)
        (Rendering|SetActorHiddenInGame (Variables|Default|GetE) false)))))

(event Custom|CheckHasMushroom
  ;[1 1 1] Mushroom Tutorial
  ;;[1 1 1] Check if player picked up Mushroom
  (if (Variables|Default|GetStartCheckingMushroom)
    (if (Variables|Default|GetReachedMushroomTutorial)
      (bind _asthird_person_character (Utilities|Casting|CastToThirdPersonCharacter (Game|GetPlayerCharacter 0)))
      (if (Variables|/Game/ThirdPersonBP/Blueprints/ThirdPersonCharacter.ThirdPersonCharacter_C|GethasMushroom _asthird_person_character)
        (Variables|Default|SetCheckMushroomUsed true)
        (Rendering|SetActorHiddenInGame (Variables|Default|GetE) false)))))

(event EventInteract
  (if (not (Variables|Default|GetIsTeleporting))
    (Utilities|FlowControl|Sequence
      (:then_0
        (if (not (Variables|Default|GetFinishedCicadaTutorial))
          ;[1 1 1] Cicada Tutorial
          (if (Variables|Default|GetReachedCicadaTutorial)
            (if (Variables|Default|GetUsedCicada)
              (Variables|Default|SetLineCurrent 1)
              (Variables|Default|SetConversation_ID 5)
              (Utilities|FlowControl|Delay 0.2)
              (Variables|Default|SetReachedMushroomTutorial true)
              (Variables|Default|SetFinishedCicadaTutorial true)
              (Utilities|Time|ClearTimerbyFunctionName 0 "CheckHasCicada")
              (Utilities|Time|ClearTimerbyFunctionName 0 "CheckUsedCicada")
              (Variables|Default|SetIsTeleporting true)
              (Utilities|FlowControl|Delay 4.0)
              (Transformation|SetWorldLocation (Variables|Collision|GetCapsuleComponent) (Transformation|GetWorldLocation (Variables|/Script/Engine.Actor|GetRootComponent (Variables|Default|GetLocation1))) false false)
              (Variables|Default|SetIsTeleporting false)
              (elif (Variables|Default|GetCicadaAlreadySpawned)
                _
                (else
                  (bind _returnvalue (Game|SpawnActorfromClass "/Game/Blueprints/Items/DroppedItem.DroppedItem_C" (Transformation|GetWorldTransform (Variables|Default|GetItemDropLoc)) "AlwaysSpawn" 0 0))
                  (Variables|/Game/Blueprints/Items/DroppedItem.DroppedItem_C|SetItem _returnvalue 3)
                  (Variables|Default|SetCicadaAlreadySpawned true)
                  (Variables|Default|SetStartCheckingCicada true))))
            (Math|Integer|IncrementInt (Variables|Default|GetLineCurrent) :!label _label
              (:%20%20
                (CallFunction|DialogueCreate)
                ;[1 1 1] When talking to NPC, this sets npc to face the player
                (Transformation|SetActorRotation (Math|Rotator|MakeRotator 0.0 0.0 (.Yaw (Math|Rotator|BreakRotator (Math|Rotator|FindLookatRotation (Transformation|GetActorLocation) (Transformation|GetActorLocation (Game|GetPlayerCharacter 0))))))))))))
      (:then_1
        (if (Variables|Default|GetFinishedIronBodyTutorial)
          (goto _label)
          (else
            ;[1 1 1] Iron Body Tutorial
            (if (Variables|Default|GetReachedIronBodyTutorial)
              (if (Variables|Default|GetUsedIronBody)
                (Utilities|FlowControl|Delay 0.1)
                (Variables|Default|SetFinishedIronBodyTutorial true)
                (Utilities|Time|ClearTimerbyFunctionName 0 "CheckHasIronBody")
                (Utilities|Time|ClearTimerbyFunctionName 0 "CheckUsedIronBody")
                (Rendering|SetActorHiddenInGame (Variables|Default|GetE) true)
                (goto _label)
                (elif (Variables|Default|GetIronBodyAlreadySpawned)
                  (goto _label)
                  (else
                    (bind _returnvalue_2 (Game|SpawnActorfromClass "/Game/Blueprints/Items/DroppedItem.DroppedItem_C" (Transformation|GetWorldTransform (Variables|Default|GetItemDropLoc)) "AlwaysSpawn" 0 0))
                    (Variables|/Game/Blueprints/Items/DroppedItem.DroppedItem_C|SetItem _returnvalue_2 1)
                    (Variables|Default|SetIronBodyAlreadySpawned true)
                    (Variables|Default|SetStartCheckingIronBody true)
                    (goto _label))))))))
      (:then_2
        (if (not (Variables|Default|GetFinishedMushroomTutorial))
          ;[1 1 1] Mushroom Tutorial
          (if (Variables|Default|GetReachedMushroomTutorial)
            (if (Variables|Default|GetUsedMushroom)
              (Variables|Default|SetLineCurrent 1)
              (Variables|Default|SetConversation_ID 4)
              (Utilities|FlowControl|Delay 0.1)
              (Variables|Default|SetReachedIronBodyTutorial true)
              (Variables|Default|SetFinishedMushroomTutorial true)
              (Utilities|Time|ClearTimerbyFunctionName 0 "CheckHasMushroom")
              (Utilities|Time|ClearTimerbyFunctionName 0 "CheckUsedMushroom")
              (Variables|Default|SetIsTeleporting true)
              (Utilities|FlowControl|Delay 4.0)
              (Transformation|SetWorldLocation (Variables|Collision|GetCapsuleComponent) (Transformation|GetWorldLocation (Variables|/Script/Engine.Actor|GetRootComponent (Variables|Default|GetLocation2))) false false)
              (Variables|Default|SetIsTeleporting false)
              (goto _label)
              (elif (Variables|Default|GetMushroomAlreadySpawned)
                (goto _label)
                (else
                  (bind _returnvalue_3 (Game|SpawnActorfromClass "/Game/Blueprints/Items/DroppedItem.DroppedItem_C" (Transformation|GetWorldTransform (Variables|Default|GetItemDropLoc)) "AlwaysSpawn" 0 0))
                  (Variables|/Game/Blueprints/Items/DroppedItem.DroppedItem_C|SetItem _returnvalue_3 4)
                  (Variables|Default|SetMushroomAlreadySpawned true)
                  (Variables|Default|SetStartCheckingMushroom true)
                  (goto _label))))))))))

(event EventBeginPlay
  ;[1 1 1] Gets all dialogue llines based on npc id num
  (bind _outrownames (DataTable|GetDataTableRowNames "/Game/Blueprints/Dialogue/Dialogue.Dialogue"))
  (for _array_element _outrownames
    (bind _returnvalue (Utilities|GetDataTableRow "/Game/Blueprints/Dialogue/Dialogue.Dialogue" _array_element)
      (:then
        (if (== (.NPC_ID (Utilities|Struct|BreakDialogueStructure _returnvalue)) (Variables|Default|GetNPC_ID))
          (Utilities|Array|Add (Variables|Default|GetDialogue) _array_element)
          ;[1 1 1] Checks for items if they are used or have been picked up
          (Utilities|Time|SetTimerbyFunctionName 0 "CheckHasIronBody" 0.01 true)
          (Utilities|Time|SetTimerbyFunctionName 0 "CheckUsedIronBody" 0.01 true)
          (Utilities|Time|SetTimerbyFunctionName 0 "CheckHasMushroom" 0.01 true)
          (Utilities|Time|SetTimerbyFunctionName 0 "CheckUsedMushroom" 0.01 true)
          (Utilities|Time|SetTimerbyFunctionName 0 "CheckHasCicada" 0.01 true)
          (Utilities|Time|SetTimerbyFunctionName 0 "CheckUsedCicada" 0.01 true))))))

(fn ConstructionScript)

(fn DialogueCreate
  (Utilities|IsValid (Variables|Default|GetDialogueWidget)
    (:Is%20Valid
      (bind _returnedline (CallFunction|DialogueGetLine))
      (if (Utilities|Enum|NotEqual(Enum) _returnedline (Variables|Default|GetEmptyText))
        (Variables|/Game/UI/Widgets/Dialogue.Dialogue_C|SetDialogueText (Variables|Default|GetDialogueWidget) _returnedline)
        (Development|PrintString "Dialogue Changed")))
    (:Is%20Not%20Valid
      (bind _returnvalue (UserInterface|CreateWidget "/Game/UI/Widgets/Dialogue.Dialogue_C" (Game|GetPlayerController 0)))
      (bind _output_get (Variables|Default|SetDialogueWidget _returnvalue))
      (UserInterface|Viewport|AddtoViewport _output_get 0)
      (bind _returnedline_2 (CallFunction|DialogueGetLine))
      (Utilities|IsValid (Variables|Default|GetDialogueWidget)
        (:Is%20Valid
          (Variables|/Game/UI/Widgets/Dialogue.Dialogue_C|SetDialogueText (Variables|Default|GetDialogueWidget) _returnedline_2)
          (Development|PrintString "Dialogue created"))))))

(fn DialogueGetLine
  (for _array_element (Variables|Default|GetDialogue)
    (bind _returnvalue (Utilities|GetDataTableRow "/Game/Blueprints/Dialogue/Dialogue.Dialogue" _array_element)
      (:then
        (if (and (== (.Conversation_ID (Utilities|Struct|BreakDialogueStructure _returnvalue)) (Variables|Default|GetConversation_ID)) (== (.Line_ID (Utilities|Struct|BreakDialogueStructure _returnvalue)) (Variables|Default|GetLineCurrent)))
          (Utilities|Array|Add (LocalVariables|GetReturnedLines) (.Dialogue (Utilities|Struct|BreakDialogueStructure _returnvalue)))))))
  (if (== (Utilities|Array|Length (LocalVariables|GetReturnedLines)) 1)
    (return (Utilities|Array|Get(acopy) (LocalVariables|GetReturnedLines)))
    (else
      (Widget|RemovefromParent (Variables|Default|GetDialogueWidget))
      (Variables|Default|SetDialogueWidget 0)
      (Variables|Default|SetLineCurrent 0))))