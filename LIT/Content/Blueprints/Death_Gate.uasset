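; Death_Gate is a gate actor that reacts when a LightProjectile hits its Cube3 component.
; On overlap it destroys the projectile and permanently adds to Cube4's vertical scale, so the growth accumulates with each hit.
; Two chained MoveComponentTo calls then drop Cube4 with no set duration and raise it by the same distance over a few seconds.
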(event OnComponentBeginOverlap(Cube3)
  (params (OverlappedComponent :type Primitive%20Component%20Object%20Reference) (OtherActor :type Actor%20Object%20Reference) (OtherComp :type Primitive%20Component%20Object%20Reference) (OtherBodyIndex :type Integer) (bFromSweep :type Boolean) (SweepResult :type Hit%20Result%20Structure%20%28by%20ref%29))
  (bind _cube4 (Variables|Default|GetCube4))
  (bind _relativelocation (Variables|/Script/Engine.SceneComponent|GetRelativeLocation _cube4))
  (bind _aslight_projectile (Utilities|Casting|CastToLightProjectile OtherActor))
  (Actor|DestroyActor _aslight_projectile)
  (Transformation|SetWorldScale3D _cube4 (+ (Transformation|GetWorldScale _cube4) "0, 0,1.000000"))
  (Components|MoveComponentTo _cube4 (- _relativelocation "0, 0,250.000000") "0, 0, 0" false false 0.2 false)
  (Components|MoveComponentTo _cube4 (+ _relativelocation "0, 0,250.000000") "0, 0, 0" false false 3.0 false))

(event EventBeginPlay)

(event EventTick
  (params (DeltaSeconds :type Float%20%28single-precision%29)))

(fn ConstructionScript)