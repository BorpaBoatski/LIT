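; Test actor Blueprint that spins continuously around its vertical axis, named as a spinning spot light.
; BeginPlay seeds ElapsedTime with the actor's current yaw, so the variable holds an angle despite its name.
; Tick advances it at a fixed, frame-rate independent rate and applies it as absolute yaw, keeping roll and pitch and never wrapping the value.
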(event EventTick
  (params (DeltaSeconds :type Float%20%28single-precision%29))
  (bind _returnvalue (Transformation|GetActorRotation))
  (bind (_roll _pitch) (Math|Rotator|BreakRotator _returnvalue))
  (bind _output_get (Variables|Default|SetElapsedTime (+ (Variables|Default|GetElapsedTime) (* DeltaSeconds 1e+02))))
  (Transformation|SetActorRotation (Math|Rotator|MakeRotator _roll _pitch _output_get)))

(event EventBeginPlay
  (Variables|Default|SetElapsedTime (.Yaw (Math|Rotator|BreakRotator (Transformation|GetActorRotation)))))

(fn ConstructionScript)