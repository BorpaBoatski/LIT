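; A debug teleporter actor that moves the player character between a Home point and an Area point.
; Overlapping either point with the ThirdPersonCharacter enables input and sets the direction; leaving disables it.
; Pressing E then sets the player's location to the opposite point.
; Two text renders rotate every tick to face the player, one showing the AreaName set at BeginPlay.
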(event OnComponentBeginOverlap(Home)
  (params (OverlappedComponent :type Primitive%20Component%20Object%20Reference) (OtherActor :type Actor%20Object%20Reference) (OtherComp :type Primitive%20Component%20Object%20Reference) (OtherBodyIndex :type Integer) (bFromSweep :type Boolean) (SweepResult :type Hit%20Result%20Structure%20%28by%20ref%29))
  (Utilities|Casting|CastToThirdPersonCharacter OtherActor)
  (Input|EnableInput (Game|GetPlayerController 0))
  (Variables|Default|SetToArea true))

(event OnComponentEndOverlap(Home)
  (params (OverlappedComponent :type Primitive%20Component%20Object%20Reference) (OtherActor :type Actor%20Object%20Reference) (OtherComp :type Primitive%20Component%20Object%20Reference) (OtherBodyIndex :type Integer))
  (Utilities|Casting|CastToThirdPersonCharacter OtherActor)
  (Input|DisableInput (Game|GetPlayerController 0)))

(event OnComponentBeginOverlap(Area)
  (params (OverlappedComponent :type Primitive%20Component%20Object%20Reference) (OtherActor :type Actor%20Object%20Reference) (OtherComp :type Primitive%20Component%20Object%20Reference) (OtherBodyIndex :type Integer) (bFromSweep :type Boolean) (SweepResult :type Hit%20Result%20Structure%20%28by%20ref%29))
  (Utilities|Casting|CastToThirdPersonCharacter OtherActor)
  (Input|EnableInput (Game|GetPlayerController 0))
  (Variables|Default|SetToArea false))

(event OnComponentEndOverlap(Area)
  (params (OverlappedComponent :type Primitive%20Component%20Object%20Reference) (OtherActor :type Actor%20Object%20Reference) (OtherComp :type Primitive%20Component%20Object%20Reference) (OtherBodyIndex :type Integer))
  (Utilities|Casting|CastToThirdPersonCharacter OtherActor)
  (Input|DisableInput (Game|GetPlayerController 0)))

(event EventBeginPlay
  (Variables|Default|SetPlayer (Game|GetPlayerCharacter 0))
  (Rendering|Components|TextRender|SetText (Variables|Default|GetTextRender1) (Variables|Default|GetAreaName)))

(event EventTick
  (params (DeltaSeconds :type Float%20%28single-precision%29))
  (bind _textrender (Variables|Default|GetTextRender))
  (bind _player (Variables|Default|GetPlayer))
  (bind _textrender1 (Variables|Default|GetTextRender1))
  (bind _returnvalue (Transformation|GetActorLocation _player))
  (Transformation|SetWorldRotation _textrender (Math|Rotator|FindLookatRotation (Transformation|GetWorldLocation _textrender) _returnvalue) false false)
  (Transformation|SetWorldRotation _textrender1 (Math|Rotator|FindLookatRotation (Transformation|GetWorldLocation _textrender1) _returnvalue) false false))

(event Input|KeyboardEvents|E
  (params (Key :type Key%20Structure))
  (:Pressed
    (if (Variables|Default|GetToArea)
      (Transformation|SetActorLocation (Variables|Default|GetPlayer) (Transformation|GetWorldLocation (Variables|Default|GetArea)) false false)
      (else
        (Transformation|SetActorLocation (Variables|Default|GetPlayer) (Transformation|GetWorldLocation (Variables|Default|GetHome)) false false)))))

(fn ConstructionScript)